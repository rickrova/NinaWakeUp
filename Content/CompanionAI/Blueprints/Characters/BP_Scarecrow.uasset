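; BP_Scarecrow is a physics-driven damageable scarecrow that shows its health as debug text.
; While health remains, damage lowers it and applies a radial impulse to the Scarecrow component from the damage causer's location.
; When health reaches zero, the physics constraint is destroyed, releasing the body.
; Each hit enables Tick to draw the health text, and a retriggerable delay switches Tick off a few seconds after the last hit.
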(event Game|Damage|EventAnyDamage
  (params (Damage :type Float%20%28single-precision%29) (DamageType :type Damage%20Type%20Object%20Reference) (InstigatedBy :type Controller%20Object%20Reference) (DamageCauser :type Actor%20Object%20Reference))
  ;[0 0 0] Damage & Death
  (if (> (Variables|Default|GetHealth) 0.0)
    (Utilities|FlowControl|Sequence
      (:then_0
        (bind _output_get (Variables|Default|SetHealth (- (Variables|Default|GetHealth) Damage)))
        (Physics|AddRadialImpulse (Variables|Default|GetScarecrow) (Transformation|GetActorLocation DamageCauser) 3e+02 5e+02 "RIF_Constant" true)
        (if (<= _output_get 0.0)
          (Components|DestroyComponent (Variables|Default|GetPhysicsConstraint))))
      (:then_1
        ;[0.903 0 1] Enable tick for debug health
        (Actor|Tick|SetActorTickEnabled true)
        (Utilities|FlowControl|RetriggerableDelay 3.0)
        (Actor|Tick|SetActorTickEnabled false)))))

(event EventTick
  (params (DeltaSeconds :type Float%20%28single-precision%29))
  ;[1 0 0.9981] Show debug health
  (Rendering|Debug|DrawDebugString (Transformation|GetWorldLocation (Variables|Default|GetDebug%20Text%20Location)) (Utilities|String|Append "Health: " (Utilities|String|ToString(Integer) (Math|Float|Round (Variables|Default|GetHealth)))) 0 "(R=1.000000,G=0.000000,B=0.017520,A=1.000000)"))

(fn ConstructionScript)