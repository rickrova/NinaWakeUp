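; Base companion character that follows its master, waits at a pointed location, attacks an enemy, and fetches and drops objects.
; Command events set a state enum and targets on the AI controller's Blackboard.
; Attack plays a montage, applies damage and returns to follow.
; Grabbing attaches the object to a mesh socket, optionally timed by a montage notify, and reverts to follow if BP_Player already holds that object.
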(event Custom|Attack
  ;[0 0 0] Basic attack logic
  (Animation|Montage|PlayMontage (Variables|Character|GetMesh) (Variables|Animaiton|GetAttack%20Montage)
    (:then
      (Game|Damage|ApplyDamage (Variables|CompanionData|GetTargeted%20Enemy) (Variables|CompanionData|GetAttack%20damage) 0 self)
      (CallFunction|UpdateState "NewEnumerator1"))))

(event Custom|Wait
  (params (Pointing%20location :type Vector))
  ;[0 0 0] Wait
  (CallFunction|UpdateState "NewEnumerator1") ; Cancel all other states
  (CallFunction|UpdateState "NewEnumerator0")
  (AI|Components|Blackboard|SetValueasVector (Variables|Default|GetBlackboard) (Utilities|Name|MakeLiteralName "Waiting Location") Pointing%20location))

(event Custom|Grab%20object
  (bind _object_to_grab (Variables|Default|GetObject%20to%20grab))
  ;[0 0 0] Grab object
  (|CancelgrabifBP_Playerisholdingobjectinhand ; Change this if you are using another player blueprint
    (:OutputPin
      (if (Variables|Animaiton|GetUse%20animations%20for%20grab?)
        (Animation|Montage|PlayMontage (Variables|Character|GetMesh) (Variables|Animaiton|GetGrab%20Montage)
          (:OnNotifyBegin
            _)))
      (Physics|SetSimulatePhysics _object_to_grab false)
      (Transformation|AttachComponentToComponent _object_to_grab (Variables|Character|GetMesh) (Variables|CompanionData|GetGrab%20object%20socket) "SnapToTarget" "SnapToTarget" "KeepRelative" true)
      (AI|Components|Blackboard|SetValueasBool (Variables|Default|GetBlackboard) (Utilities|Name|MakeLiteralName "Grabbed object?") true))))

(event Custom|Start%20Combat
  (params (Enemy%20Target :type Actor%20Object%20Reference))
  ;[0 0 0] Start combat
  (Variables|CompanionData|SetTargeted%20Enemy Enemy%20Target)
  (CallFunction|UpdateState "NewEnumerator2")
  (AI|Components|Blackboard|SetValueasObject (Variables|Default|GetBlackboard) (Utilities|Name|MakeLiteralName "Attack target") Enemy%20Target))

(event Custom|Follow
  ;[0 0 0] Follow
  (CallFunction|UpdateState "NewEnumerator1"))

(event Custom|Fetch
  (params (Component :type Primitive%20Component%20Object%20Reference))
  ;[0 0 0] Fetch object
  (Variables|Default|SetObject%20to%20grab Component)
  (CallFunction|UpdateState "NewEnumerator3"))

(event Custom|Drop%20object
  (bind _object_to_grab (Variables|Default|GetObject%20to%20grab))
  ;[0 0 0] Drop object
  (if (Variables|Animaiton|GetUse%20animations%20for%20grab?)
    (Animation|Montage|PlayMontage (Variables|Character|GetMesh) "/Game/CompanionAI/Characters/Dog/Dog_Grab_Montage.Dog_Grab_Montage"
      (:then
        _)))
  (Transformation|DetachFromComponent _object_to_grab "KeepRelative" "KeepRelative" "KeepRelative" true)
  (Physics|SetSimulatePhysics _object_to_grab true)
  (AI|Components|Blackboard|SetValueasBool (Variables|Default|GetBlackboard) (Utilities|Name|MakeLiteralName "Grabbed object?") false)
  (CallFunction|UpdateState "NewEnumerator1"))

(event EventBeginPlay
  (bind _master (Variables|CompanionData|GetMaster))
  ;[0 0 0] Begin play
  (Utilities|IsValid _master
    (:Is%20Valid
      (bind _output_get (Variables|Default|SetBlackboard (AI|GetBlackboard (Pawn|GetController))))
      (AI|Components|Blackboard|SetValueasObject _output_get (Utilities|Name|MakeLiteralName "Master") _master))))

(fn ConstructionScript)

(fn UpdateState
  (params (Desired%20State :type Enum_CompanionState%20Enum :default "NewEnumerator0"))
  (bind _output_get (Variables|CompanionData|SetCurrent%20state Desired%20State))
  (AI|Components|Blackboard|SetValueasEnum (Variables|Default|GetBlackboard) (Utilities|Name|MakeLiteralName "State") _output_get))