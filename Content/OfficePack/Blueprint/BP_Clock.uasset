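; BP_Clock is a clock prop whose hands show the current time returned by Now.
; On every Tick it sets the relative yaw of the HourHand, MinuteHand and SecondHand components from that time.
; The hour and minute hands include the smaller time units so they creep between marks, while the second hand steps in whole seconds.
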(event EventTick
  (params (DeltaSeconds :type Float%20%28single-precision%29))
  (bind _returnvalue (Math|DateTime|Now))
  (bind _returnvalue_2 (Class|KismetMathLibrary|GetMinute _returnvalue))
  (bind _returnvalue_3 (Class|KismetMathLibrary|GetSecond _returnvalue))
  (bind _returnvalue_4 (Math|Conversions|ToFloat(Integer) _returnvalue_3))
  (Transformation|SetRelativeRotation (Variables|Default|GetHourHand) (Math|Rotator|MakeRotator 0.0 0.0 (* (+ (* (+ (* (Class|KismetMathLibrary|GetHour12 _returnvalue) 6e+01) (Math|Conversions|ToFloat(Integer) _returnvalue_2)) 6e+01) _returnvalue_4) 0.0083333)) false false)
  (Transformation|SetRelativeRotation (Variables|Default|GetMinuteHand) (Math|Rotator|MakeRotator 0.0 0.0 (* (+ _returnvalue_4 (* _returnvalue_2 6e+01)) 0.1)) false false)
  (Transformation|SetRelativeRotation (Variables|Default|GetSecondHand) (Math|Rotator|MakeRotator 0.0 0.0 (* _returnvalue_3 6.0)) false false))

(fn ConstructionScript)