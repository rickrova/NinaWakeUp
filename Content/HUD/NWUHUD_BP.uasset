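; HUD Blueprint that creates the main Frame widget and drives inventory UI and 3D item inspection.
; It forwards navigation, cursor, prompt-panel, inventory and camera-transition events to the widget.
; Inspection adds a static or skeletal mesh component to a camera actor spawned far below the world and switches the view to it with post-processing.
; Input rotates, pans and FOV-zooms the item; closing destroys it and restores the previous camera.
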(event Custom|Out
  (CallFunction|SwitchPromptRequest "NewEnumerator5" (stale EventSwitchPromptRequest In) false))

(event Custom|UnlockDraw
  (params (InIndex :type Integer))
  (Utilities|Array|Add (Variables|Default|GetDrawsIndices) InIndex))

(event Custom|CameraTransition
  (bind _alpha (Timeline|Timeline PlayFromStart)
    (:Update
      (Default|UpdateCameraTransition (Variables|Default|GetCanvasContainer) _alpha))))

(event Custom|SwitchCursor
  (Default|SwitchCursor (Variables|Default|GetCanvasContainer)))

(event EventBeginPlay
  (bind _returnvalue (UserInterface|CreateWidget "/Game/HUD/Frame.Frame_C"))
  (bind _output_get (Variables|Default|SetCanvasContainer _returnvalue))
  (UserInterface|Viewport|AddtoPlayerScreen _output_get)
  (Default|CallOnUICreated)
  (Default|Init (Variables|Default|GetCanvasContainer))
  (CallFunction|SpawnInspectCamera))

(event EventSwitchPanelVisibility
  (params (InTypeID :type Integer) (OutTypeID :type Integer))
  (Default|SwitchPanels (Variables|Default|GetCanvasContainer) (Utilities|Array|MakeArray (Utilities|Enum|ByteToEnumPromptType (Math|Conversions|ToByte(Integer) InTypeID))) (Utilities|Array|MakeArray (Utilities|Enum|ByteToEnumPromptType (Math|Conversions|ToByte(Integer) OutTypeID)))))

(event EventDown
  (Default|SelectDown (Variables|Default|GetCanvasContainer)))

(event EventUp
  (Default|SelectUp (Variables|Default|GetCanvasContainer)))

(event EventAccept
  (Default|Accept (Variables|Default|GetCanvasContainer)))

(event EventCancel
  (Default|Cancel (Variables|Default|GetCanvasContainer)))

(event EventCloseInspect
  (CallFunction|CloseInspectPanel))

(event EventCloseInspectMesh
  (CallFunction|CloseInspectPanel))

(event EventNextPage
  (Class|ItemImputBridge|PadRight(Message) (Variables|Default|GetInspectedMesh)))

(event EventPrevPage
  (Class|ItemImputBridge|PadLeft(Message) (Variables|Default|GetInspectedMesh)))

(event EventPanItem
  (params (Value :type Vector%202D%20Structure))
  (Variables|Default|SetItemOffset (Class|KismetMathLibrary|ClampAxes2D (+ (Variables|Default|GetItemOffset) (* Value "(X=0.500000,Y=0.500000)")) -1e+01 1e+01)))

(event EventMoveCursorHorizontal
  (params (Value :type Float%20%28single-precision%29))
  (Default|MoveCursor (Variables|Default|GetCanvasContainer) (Math|Vector2D|MakeVector2D Value (stale EventMoveCursorVertical Value))))

(event EventInspect
  (params (InType :type Mesh%20Component%20Class%20Reference) (InStaticMesh :type Static%20Mesh%20Object%20Reference) (InSkeletalMesh :type Skeletal%20Mesh%20Object%20Reference))
  (CallFunction|ShowInspectPanel InType InStaticMesh InSkeletalMesh))

(event EventRollItem
  (params (Value :type Float%20%28single-precision%29))
  ;[1 1 1] Item Inspect
  (bind _output_get (Variables|Default|SetAnalogueMovement (Math|Vector|MakeVector (.x (Variables|Default|GetAnalogueMovement)) (.y (Variables|Default|GetAnalogueMovement)) Value)))
  (CallFunction|RotateItem _output_get (Variables|Default|GetZoom) (Variables|Default|GetItemOffset)))

(event EventZoomItem
  (params (Value :type Float%20%28single-precision%29))
  ;[1 1 1] Item Inspect
  (bind _output_get (Variables|Default|SetZoom (Math|Float|Clamp(Float) (- (Variables|Default|GetZoom) (* Value 0.1)) -1.0)))
  (CallFunction|RotateItem (Variables|Default|GetAnalogueMovement) _output_get (Variables|Default|GetItemOffset)))

(event EventMoveCursorVertical
  (params (Value :type Float%20%28single-precision%29))
  (Default|MoveCursor (Variables|Default|GetCanvasContainer) (Math|Vector2D|MakeVector2D (stale EventMoveCursorHorizontal Value) Value)))

(event EventUpdateInventory
  (params (inItem :type Item%20Meta%20Structure))
  (Default|AddItemtoInventory (Variables|Default|GetCanvasContainer) inItem))

(event EventSwitchPromptRequest
  (params (In :type PromptType%20Enum :default "NewEnumerator5") (Out :type PromptType%20Enum :default "NewEnumerator5") (Temp :type Boolean))
  (Default|SwitchPanels (Variables|Default|GetCanvasContainer) (Utilities|Array|MakeArray In) (Utilities|Array|MakeArray Out))
  (if Temp
    (Utilities|Time|SetTimerbyEvent (delegate Custom|Out) 2.0)))

(event EventVertical
  (params (Value :type Float%20%28single-precision%29))
  ;[1 1 1] Item Inspect
  (Variables|Default|SetAnalogueMovement (Math|Vector|MakeVector (.x (Variables|Default|GetAnalogueMovement)) Value (.z (Variables|Default|GetAnalogueMovement)))))

(event EventHorizontal
  (params (Value :type Float%20%28single-precision%29))
  ;[1 1 1] Item Inspect
  (Variables|Default|SetAnalogueMovement (Math|Vector|MakeVector Value (.y (Variables|Default|GetAnalogueMovement)) (.z (Variables|Default|GetAnalogueMovement)))))

(event EventSwitchInventoryVisibility
  (Default|ShowInventory (Variables|Default|GetCanvasContainer))
  (Development|PrintString "show inventory"))

(event EventRight
  (Default|SelectNext (Variables|Default|GetCanvasContainer)))

(event EventLeft
  (Default|SelectPrevious (Variables|Default|GetCanvasContainer)))

(fn ConstructionScript)

(fn SpawnInspectCamera
  (bind _returnvalue (Game|SpawnActorfromClass "/Game/Blueprints/CameraSystemF/InspectCamera.InspectCamera_C" (Math|Transform|MakeTransform "0.000000,0.000000,-5000.000000" "0, 0, 0" "1.000000,1.000000,1.000000") "AlwaysSpawn" 0 0))
  (Variables|Default|SetInspectCamera (Actor|GetComponentbyClass _returnvalue "/Script/Engine.CameraComponent")))

(fn ShowInspectPanel
  (params (InType :type Mesh%20Component%20Class%20Reference) (InStaticMesh :type Static%20Mesh%20Object%20Reference) (InSkeletalMesh :type Skeletal%20Mesh%20Object%20Reference))
  (bind _returnvalue (Game|AddComponentbyClass (Components|GetOwner (Variables|Default|GetInspectCamera)) InType false (Math|Transform|MakeTransform "40.000000,0.000000,0.000000" "0, 0, 0" "1.000000,1.000000,1.000000")))
  (bind _output_get (Variables|Default|SetInspectedMesh _returnvalue))
  (if (!= InStaticMesh 0)
    (bind _asstatic_mesh_component (Utilities|Casting|CastToStaticMeshComponent _output_get))
    (Utilities|IsValid InStaticMesh
      (:Is%20Valid
        (Components|StaticMesh|SetStaticMesh _asstatic_mesh_component InStaticMesh))
      (:Is%20Not%20Valid
        _))
    (Development|PrintString "static")
    (else
      (bind _asskeletal_mesh_component (Utilities|Casting|CastToSkeletalMeshComponent _output_get))
      (Utilities|IsValid InSkeletalMesh
        (:Is%20Valid
          (Components|SkeletalMesh|SetSkeletalMeshAsset _asskeletal_mesh_component InSkeletalMesh))
        (:Is%20Not%20Valid
          _))
      (Development|PrintString "skeletal")))
  (Rendering|SetVisibility (Variables|Default|GetInspectedMesh) true true)
  (Collision|SetCollisionResponsetoAllChannels (Variables|Default|GetInspectedMesh) "ECR_Ignore")
  (Rendering|SetRenderCustomDepth (Variables|Default|GetInspectedMesh) true)
  (Transformation|SetMobility (Variables|Default|GetInspectedMesh) "Movable")
  (bind _asnina_character_bp (Utilities|Casting|CastToNinaCharacter_BP (Game|GetPlayerCharacter 0)))
  (Variables|Default|SetPreviousCamera (Variables|/Script/NinaProject.BaseCharacter|GetCurrentCamera _asnina_character_bp))
  (Game|Player|SetViewTargetwithBlend (Game|GetPlayerController 0) (Components|GetOwner (Variables|Default|GetInspectCamera)) 0.0 "VTBlend_Linear" 0.0 false)
  (Transformation|SetRelativeRotation (Variables|Default|GetInspectedMesh) "0.000000,90.000000,90.000000" false false)
  (Variables|Default|SetZoom 0.0)
  (Variables|Default|SetItemOffset "")
  (bind _asnwugame_mode (Utilities|Casting|CastToNWUGameMode (Game|GetGameMode)))
  (Default|DisableThisCamera (Variables|/Game/Blueprints/NWUGameMode.NWUGameMode_C|GetCurrentCamera _asnwugame_mode))
  (Variables|/Script/Engine.PostProcessComponent|SetbEnabled (Actor|GetComponentbyClass (Components|GetOwner (Variables|Default|GetInspectCamera)) "/Script/Engine.PostProcessComponent") true))

(fn RotateItem
  (params (InRotation :type Vector) (InZoom :type Float%20%28double-precision%29) (Offset :type Vector%202D%20Structure))
  (bind _inspectedmesh (Variables|Default|GetInspectedMesh))
  (if (!= _inspectedmesh 0)
    (Transformation|AddWorldRotation _inspectedmesh (Math|Rotator|MakeRotator (.z InRotation) (.y InRotation) (.x InRotation)) false false)
    (Transformation|SetRelativeLocation _inspectedmesh (Math|Vector|MakeVector 4e+01 (.x Offset) (.y Offset)) false false)
    (Camera|SetFieldOfView (Variables|Default|GetInspectCamera) (+ (* InZoom 6e+01) 9e+01))))

(fn CloseInspectPanel
  (bind _inspectedmesh (Variables|Default|GetInspectedMesh))
  (Utilities|IsValid _inspectedmesh
    (:Is%20Valid
      (Transformation|DetachFromComponent _inspectedmesh "KeepRelative" "KeepRelative" "KeepRelative" true)
      (Components|DestroyComponent _inspectedmesh)
      (Game|Player|SetViewTargetwithBlend (Game|GetPlayerController 0) (Components|GetOwner (Variables|Default|GetPreviousCamera)) 0.0 "VTBlend_Linear" 0.0 false)
      (bind _asnwugame_mode (Utilities|Casting|CastToNWUGameMode (Game|GetGameMode)))
      (Variables|/Script/Engine.PostProcessComponent|SetbEnabled (Actor|GetComponentbyClass (Components|GetOwner (Variables|Default|GetInspectCamera)) "/Script/Engine.PostProcessComponent") false)
      (Default|SetThisCamera (Variables|/Game/Blueprints/NWUGameMode.NWUGameMode_C|GetCurrentCamera _asnwugame_mode)))))