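; Player character Blueprint for Nina, handling jumping, jetpack floating, gadget zoom, grabbing, pushing, ladder climbing, boat seating, health and collectables.
; Events forward state to Nina_Animation_BP and fire dispatchers for damage, pickups, menu selection and pause.
; Timelines animate jetpack flames, the spawned info prompt and boat seating; mid-air zoom slows time.
; A custom event writes current and trailing player positions to a material parameter collection for shader interaction.
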(event Custom|Grab
  (params (HitResult :type Hit%20Result%20Structure))
  (Class|BaseCharacter|OnGrab HitResult)
  (bind _asnina_animation_bp (CallFunction|GetAnimationBlueprint))
  (bind _output_get (Variables|/Game/Characters/Nina/Animations/Nina_Animation_BP.Nina_Animation_BP_C|SetbGrab _asnina_animation_bp true))
  (Variables|Default|SetIsGrabbing _output_get))

(event Custom|OnClimbableInteractionEnd)

(event Custom|SetMinFire
  (bind _fire2 (Variables|Default|GetFire2))
  (bind _fire (Variables|Default|GetFire))
  (bind _relativescale3d (Variables|/Script/Engine.SceneComponent|GetRelativeScale3D _fire2))
  (bind _relativescale3d_2 (Variables|/Script/Engine.SceneComponent|GetRelativeScale3D _fire))
  (bind (_direction _fireloopcurve _newtrack_2) (Timeline|Timeline_2 PlayFromStart)
    (:Update
      (Transformation|SetRelativeScale3D _fire (Math|Vector|MakeVector (.x _relativescale3d_2) (.y _relativescale3d_2) (* _fireloopcurve (Variables|Default|GetMinFireScale))))
      (Transformation|SetRelativeScale3D _fire2 (Math|Vector|MakeVector (.x _relativescale3d) (.y _relativescale3d) (* _newtrack_2 (Variables|Default|GetMinFireScale)))))))

(event Custom|ResetInvincible
  (Variables|Default|SetbInvincible false)
  (Class|BaseCharacter|BlinkMaterial)
  (bind _ashazard_bp (Utilities|Casting|CastToHazard_BP (stale Custom|OnDamage Other)))
  (Default|CheckDamage _ashazard_bp))

(event Custom|FloatGate
  (bind _fire2 (Variables|Default|GetFire2))
  (bind _fire (Variables|Default|GetFire))
  (bind _relativescale3d (Variables|/Script/Engine.SceneComponent|GetRelativeScale3D _fire2))
  (bind _relativescale3d_2 (Variables|/Script/Engine.SceneComponent|GetRelativeScale3D _fire))
  (bind (_direction _fireloopcurve _newtrack_2) (Timeline|Timeline_2 Stop)
    (:Update
      (Transformation|SetRelativeScale3D _fire (Math|Vector|MakeVector (.x _relativescale3d_2) (.y _relativescale3d_2) (* _fireloopcurve (Variables|Default|GetMinFireScale))))
      (Transformation|SetRelativeScale3D _fire2 (Math|Vector|MakeVector (.x _relativescale3d) (.y _relativescale3d) (* _newtrack_2 (Variables|Default|GetMinFireScale)))))))

(event Custom|GrabEnd
  (Class|BaseCharacter|OnGrabEnd)
  (bind _asnina_animation_bp (CallFunction|GetAnimationBlueprint))
  (bind _output_get (Variables|/Game/Characters/Nina/Animations/Nina_Animation_BP.Nina_Animation_BP_C|SetbGrab _asnina_animation_bp false))
  (Variables|Default|SetIsGrabbing _output_get))

(event Custom|BoatSeat
  (params (Seat :type Scene%20Component%20Object%20Reference))
  (bind _returnvalue (Transformation|GetWorldTransform Seat))
  (Collision|SetCollisionEnabled (Variables|Default|GetCapsuleComponent) "NoCollision")
  (Transformation|AttachComponentToComponent Seat "None" "KeepWorld" "KeepWorld" "KeepWorld" true)
  (Input|SetIgnoreMoveInput (Pawn|GetController) true)
  (bind _asnina_animation_bp (CallFunction|GetAnimationBlueprint))
  (Default|BoatSeat _asnina_animation_bp true)
  (Variables|Default|SetBoatInitialLocation (Transformation|GetActorLocation))
  (Variables|Default|SetBoatInitialRotation (Transformation|GetActorRotation))
  (bind _newtrack_0 (Timeline|BoatSitTimeline Play)
    (:Update
      (Transformation|SetActorLocation (Math|Vector|Lerp(Vector) (Variables|Default|GetBoatInitialLocation) (.location _returnvalue) _newtrack_0) false true)
      (Transformation|SetActorRotation (Math|Rotator|Lerp(Rotator) (Variables|Default|GetBoatInitialRotation) (.rotation _returnvalue) _newtrack_0 true) true))))

(event Custom|OnHealth
  (Variables|Default|SetLifeUnits (Math|Integer|Clamp(Integer) (+ (Variables|Default|GetLifeUnits) 1) 0 3))
  (Default|CallOnDamageDispatcher))

(event Custom|StopClimbLadder
  (bind _asnina_animation_bp (CallFunction|GetAnimationBlueprint))
  (Default|StopClimbLadder _asnina_animation_bp))

(event Custom|ClimbLadder
  (bind _asnina_animation_bp (CallFunction|GetAnimationBlueprint))
  (Default|ClimbLadder _asnina_animation_bp))

(event Custom|WarpLadder
  (Transformation|SetActorLocation (stale Custom|FinishClimbLadder WarpPosition) false true))

(event Custom|FinishClimbLadder
  (params (WarpPosition :type Vector))
  (bind _asnina_animation_bp (CallFunction|GetAnimationBlueprint))
  (Default|FinishClimbLadder _asnina_animation_bp))

(event Custom|OnCollect
  (Variables|Default|SetCollectableNumber (+ (Variables|Default|GetCollectableNumber) 1))
  (Default|CallCollectDispatcher))

(event Custom|ShowBackpack
  (Development|SetHiddeninGame (Variables|Default|GetBackpack) false true)
  (Physics|AddImpulse (Variables|Character|GetCharacterMovement) "0, 0,50.000000" true)
  (Variables|Default|SetbCanFloat true))

(event Custom|StartClimbLadder
  (bind _asnina_animation_bp (CallFunction|GetAnimationBlueprint))
  (Default|StartClimbLadder _asnina_animation_bp))

(event Custom|OnDamage
  (params (Other :type Actor%20Object%20Reference) (DamageAmount :type Integer))
  (bind _capsulecomponent (Variables|Default|GetCapsuleComponent))
  (bind _charactermovement (Variables|Character|GetCharacterMovement))
  (bind _hitparticles (Variables|Default|GetHitParticles))
  (bind _capsulecomponent_2 (Variables|Default|GetCapsuleComponent))
  (Variables|Default|SetLifeUnits (- (Variables|Default|GetLifeUnits) DamageAmount))
  (Transformation|SetWorldLocation _hitparticles (+ (* (Math|Vector|GetForwardVector _capsulecomponent) 5e+01) (Transformation|GetWorldLocation _capsulecomponent)) false true)
  (Components|Activation|Activate _hitparticles true)
  (Variables|/Script/Engine.MovementComponent|SetVelocity _charactermovement "0, 0, 0")
  (Physics|AddImpulse _charactermovement (- (* (Math|Vector|GetUpVector _capsulecomponent_2) 10000) (* (Math|Vector|GetForwardVector _capsulecomponent_2) (Variables|Default|GetDamageImpulse))) false)
  (Default|CallOnDamageDispatcher)
  (if (> (Variables|Default|GetLifeUnits) 0)
    (Variables|Default|SetbInvincible true)
    (Utilities|Time|SetTimerbyEvent (delegate Custom|ResetInvincible) 1.0)
    (else
      (Variables|Default|SetbKO true)
      (bind _asnina_animation_bp (CallFunction|GetAnimationBlueprint))
      (Variables|/Game/Characters/Nina/Animations/Nina_Animation_BP.Nina_Animation_BP_C|SetKO _asnina_animation_bp true)
      (Input|SetIgnoreMoveInput (Pawn|GetController) true)))
  (bind _asbase_player_controller (Utilities|Casting|CastToBasePlayerController (Pawn|GetController)))
  (Game|Feedback|PlayDynamicForceFeedback _asbase_player_controller 0.5 0.25 true true true true))

(event Custom|BoatEnd
  (Transformation|DetachFromComponent (Variables|Default|GetCapsuleComponent) "KeepWorld" "KeepWorld" "KeepWorld" true)
  (Collision|SetCollisionEnabled (Variables|Default|GetCapsuleComponent) "QueryAndPhysics")
  (Input|SetIgnoreMoveInput (Pawn|GetController) false)
  (bind _asnina_animation_bp (CallFunction|GetAnimationBlueprint))
  (Default|BoatSeat _asnina_animation_bp false))

(event Custom|OnClimbableInteractionResponse)

(event Custom|CustomEvent
  (params (DeltaSeconds :type Float%20%28double-precision%29))
  (bind _self self)
  (bind _pathlength (Variables|Default|GetPathLength))
  (bind _returnvalue (Transformation|GetActorLocation _self))
  (bind _returnvalue_2 (Transformation|GetActorForwardVector _self))
  (bind _capsulecomponent (Variables|/Script/Engine.Character|GetCapsuleComponent _self))
  (bind _returnvalue_3 (Math|Conversions|ToLinearColor(Vector) _returnvalue))
  (bind _returnvalue_4 (Math|Conversions|ToLinearColor(Vector) _returnvalue_2))
  (bind (_x _y _z) (Math|Vector|BreakVector _returnvalue))
  (bind _capsulehalfheight (Variables|/Script/Engine.CapsuleComponent|GetCapsuleHalfHeight _capsulecomponent))
  (bind _returnvalue_5 (/ _capsulehalfheight 2.0))
  (bind _returnvalue_6 (- _z _returnvalue_5))
  (bind _returnvalue_7 (+ _returnvalue_5 _z))
  (bind _returnvalue_8 (Math|Vector|MakeVector _x _y _returnvalue_6))
  (bind _returnvalue_9 (Math|Vector|MakeVector _x _y _returnvalue_7))
  (bind _returnvalue_10 (Math|Conversions|ToLinearColor(Vector) _returnvalue_8))
  (bind _returnvalue_11 (Math|Conversions|ToLinearColor(Vector) _returnvalue_9))
  ;[1 1 1] Base Interaction
  (Rendering|Material|SetVectorParameterValue "/Game/PN_OpenWorldFoliage/Materials/MaterialCollection.MaterialCollection" "PlayerDir0" _returnvalue_4 :!class /Script/Engine.KismetMaterialLibrary)
  (Rendering|Material|SetVectorParameterValue "/Game/PN_OpenWorldFoliage/Materials/MaterialCollection.MaterialCollection" "PlayerPos0" _returnvalue_10 :!class /Script/Engine.KismetMaterialLibrary)
  (Rendering|Material|SetVectorParameterValue "/Game/PN_OpenWorldFoliage/Materials/MaterialCollection.MaterialCollection" "PlayerPos1" _returnvalue_3 :!class /Script/Engine.KismetMaterialLibrary)
  (Rendering|Material|SetVectorParameterValue "/Game/PN_OpenWorldFoliage/Materials/MaterialCollection.MaterialCollection" "PlayerPos2" _returnvalue_11 :!class /Script/Engine.KismetMaterialLibrary)
  (if (Variables|Default|GetPath)
    (Utilities|Array|Add (Variables|Default|GetDir0) _returnvalue_4)
    (Utilities|Array|Add (Variables|Default|GetPos0) _returnvalue_10)
    (Utilities|Array|Add (Variables|Default|GetPos1) _returnvalue_3)
    (bind _returnvalue_12 (Utilities|Array|Add (Variables|Default|GetPos2) _returnvalue_11))
    (if (> _returnvalue_12 _pathlength)
      (Utilities|FlowControl|Sequence
        (:then_0
          ;[1 1 1] Path Interaction I
          (Rendering|Material|SetVectorParameterValue "/Game/PN_OpenWorldFoliage/Materials/MaterialCollection.MaterialCollection" "PlayerDir0-1" (Utilities|Array|Get(acopy) (Variables|Default|GetDir0) (- _returnvalue_12 (/ _pathlength 3))) :!class /Script/Engine.KismetMaterialLibrary)
          (Rendering|Material|SetVectorParameterValue "/Game/PN_OpenWorldFoliage/Materials/MaterialCollection.MaterialCollection" "PlayerPos0-1" (Utilities|Array|Get(acopy) (Variables|Default|GetPos0) (- _returnvalue_12 (/ _pathlength 3))) :!class /Script/Engine.KismetMaterialLibrary)
          (Rendering|Material|SetVectorParameterValue "/Game/PN_OpenWorldFoliage/Materials/MaterialCollection.MaterialCollection" "PlayerPos1-1" (Utilities|Array|Get(acopy) (Variables|Default|GetPos1) (- _returnvalue_12 (/ _pathlength 3))) :!class /Script/Engine.KismetMaterialLibrary)
          (Rendering|Material|SetVectorParameterValue "/Game/PN_OpenWorldFoliage/Materials/MaterialCollection.MaterialCollection" "PlayerPos2-1" (Utilities|Array|Get(acopy) (Variables|Default|GetPos2) (- _returnvalue_12 (/ _pathlength 3))) :!class /Script/Engine.KismetMaterialLibrary))
        (:then_1
          ;[1 1 1] Path Interaction II
          (Rendering|Material|SetVectorParameterValue "/Game/PN_OpenWorldFoliage/Materials/MaterialCollection.MaterialCollection" "PlayerDir0-2" (Utilities|Array|Get(acopy) (Variables|Default|GetDir0) (- _returnvalue_12 (/ (* _pathlength 2) 3))) :!class /Script/Engine.KismetMaterialLibrary)
          (Rendering|Material|SetVectorParameterValue "/Game/PN_OpenWorldFoliage/Materials/MaterialCollection.MaterialCollection" "PlayerPos0-2" (Utilities|Array|Get(acopy) (Variables|Default|GetPos0) (- _returnvalue_12 (/ (* _pathlength 2) 3))) :!class /Script/Engine.KismetMaterialLibrary)
          (Rendering|Material|SetVectorParameterValue "/Game/PN_OpenWorldFoliage/Materials/MaterialCollection.MaterialCollection" "PlayerPos1-2" (Utilities|Array|Get(acopy) (Variables|Default|GetPos1) (- _returnvalue_12 (/ (* _pathlength 2) 3))) :!class /Script/Engine.KismetMaterialLibrary)
          (Rendering|Material|SetVectorParameterValue "/Game/PN_OpenWorldFoliage/Materials/MaterialCollection.MaterialCollection" "PlayerPos2-2" (Utilities|Array|Get(acopy) (Variables|Default|GetPos2) (- _returnvalue_12 (/ (* _pathlength 2) 3))) :!class /Script/Engine.KismetMaterialLibrary))
        (:then_2
          ;[1 1 1] Comment
          (Rendering|Material|SetVectorParameterValue "/Game/PN_OpenWorldFoliage/Materials/MaterialCollection.MaterialCollection" "PlayerDir0-3" (Utilities|Array|Get(acopy) (Variables|Default|GetDir0) (- _returnvalue_12 (- _pathlength (/ _pathlength 10)))) :!class /Script/Engine.KismetMaterialLibrary)
          (Rendering|Material|SetVectorParameterValue "/Game/PN_OpenWorldFoliage/Materials/MaterialCollection.MaterialCollection" "PlayerPos0-3" (Utilities|Array|Get(acopy) (Variables|Default|GetPos0) (- _returnvalue_12 (- _pathlength (/ _pathlength 10)))) :!class /Script/Engine.KismetMaterialLibrary)
          (Rendering|Material|SetVectorParameterValue "/Game/PN_OpenWorldFoliage/Materials/MaterialCollection.MaterialCollection" "PlayerPos1-3" (Utilities|Array|Get(acopy) (Variables|Default|GetPos1) (- _returnvalue_12 (- _pathlength (/ _pathlength 10)))) :!class /Script/Engine.KismetMaterialLibrary)
          (Rendering|Material|SetVectorParameterValue "/Game/PN_OpenWorldFoliage/Materials/MaterialCollection.MaterialCollection" "PlayerPos2-3" (Utilities|Array|Get(acopy) (Variables|Default|GetPos2) (- _returnvalue_12 (- _pathlength (/ _pathlength 10)))) :!class /Script/Engine.KismetMaterialLibrary))
        (:then_3
          ;[1 1 1] Comment
          (Utilities|Array|RemoveIndex (Variables|Default|GetDir0) (- _returnvalue_12 (/ _pathlength 3)))
          (Utilities|Array|RemoveIndex (Variables|Default|GetPos0) (- _returnvalue_12 (/ _pathlength 3)))
          (Utilities|Array|RemoveIndex (Variables|Default|GetPos1) (- _returnvalue_12 (/ _pathlength 3)))
          (Utilities|Array|RemoveIndex (Variables|Default|GetPos2) (- _returnvalue_12 (/ _pathlength 3)))
          (Utilities|Array|RemoveIndex (Variables|Default|GetDir0) (- _returnvalue_12 (/ (* _pathlength 2) 3)))
          (Utilities|Array|RemoveIndex (Variables|Default|GetPos0) (- _returnvalue_12 (/ (* _pathlength 2) 3)))
          (Utilities|Array|RemoveIndex (Variables|Default|GetPos1) (- _returnvalue_12 (/ (* _pathlength 2) 3)))
          (Utilities|Array|RemoveIndex (Variables|Default|GetPos2) (- _returnvalue_12 (/ (* _pathlength 2) 3)))
          (Utilities|Array|RemoveIndex (Variables|Default|GetDir0) (- _returnvalue_12 (- _pathlength (/ _pathlength 10))))
          (Utilities|Array|RemoveIndex (Variables|Default|GetPos0) (- _returnvalue_12 (- _pathlength (/ _pathlength 10))))
          (Utilities|Array|RemoveIndex (Variables|Default|GetPos1) (- _returnvalue_12 (- _pathlength (/ _pathlength 10))))
          (Utilities|Array|RemoveIndex (Variables|Default|GetPos2) (- _returnvalue_12 (- _pathlength (/ _pathlength 10)))))))))

(event Collision|EventActorBeginOverlap
  (params (OtherActor :type Actor%20Object%20Reference)))

(event EventUse
  (Class|ExecutableInterfaceBP|Execute(Message) (Variables|Default|GetGadget)))

(event EventUpSelection
  (Default|CallUpSelectionDispatcher))

(event EventInteract
  (params (Hit :type Hit%20Result%20Structure) (InteractiveActor :type Actor%20Object%20Reference))
  (Class|BaseCharacter|OnInteraction Hit)
  (bind _asnina_animation_bp (Utilities|Casting|CastToNina_Animation_BP (Components|SkeletalMesh|GetAnimInstance (Variables|Character|GetMesh))))
  (Variables|/Game/Characters/Nina/Animations/Nina_Animation_BP.Nina_Animation_BP_C|SetbPushing _asnina_animation_bp true))

(event EventDownSelection
  (Default|CallDownSelectionDispatcher))

(event EventEndInteract
  (Class|BaseCharacter|OnInteractionEnd)
  (bind _asnina_animation_bp (Utilities|Casting|CastToNina_Animation_BP (Components|SkeletalMesh|GetAnimInstance (Variables|Character|GetMesh))))
  (Variables|/Game/Characters/Nina/Animations/Nina_Animation_BP.Nina_Animation_BP_C|SetbPushing _asnina_animation_bp false))

(event EventAcceptSelection
  (Default|CallAcceptSelectionDispatcher))

(event EventPause
  (params (bPause :type Boolean))
  (if bPause
    (Default|CallPauseDispatcher)
    (else
      (Default|CallUnPauseDispatcher))))

(event EventTick
  (params (DeltaSeconds :type Float%20%28single-precision%29)))

(event EventOnNinaBeginJump
  ;[1 1 1] To animation blueprin
  (bind _asnina_animation_bp (CallFunction|GetAnimationBlueprint))
  (if (not (Variables|/Game/Characters/Nina/Animations/Nina_Animation_BP.Nina_Animation_BP_C|GetbHit _asnina_animation_bp))
    (Variables|Default|SetbPendingJump true)
    (Variables|/Script/Engine.CharacterMovementComponent|SetRotationRate (Variables|Character|GetCharacterMovement) "0,100.000000, 0")
    (Default|OnStartJump _asnina_animation_bp)))

(event EventOnNinaEndJump
  ;[1 1 1] To animation blueprin
  (Variables|/Script/Engine.CharacterMovementComponent|SetRotationRate (Variables|Character|GetCharacterMovement) (Variables|Default|GetInitialRotationRate))
  (bind _asnina_animation_bp (CallFunction|GetAnimationBlueprint))
  (Default|OnEndJump _asnina_animation_bp))

(event EventShowUI
  (params (TextureIndex :type Integer))
  (bind _returnvalue (Rendering|Material|CreateDynamicMaterialInstance (Variables|/Game/Blueprints/Test/InfoActor.InfoActor_C|GetInfo (Variables|Default|GetInfoActor)) 0 "/Game/Characters/Nina/NinaInfo_Mat.NinaInfo_Mat" "None" :!class /Script/Engine.PrimitiveComponent))
  (Rendering|Material|SetTextureParameterValue _returnvalue "ButtonTexture" (Utilities|Array|Get(acopy) (Variables|Default|GetTextureArray) TextureIndex))
  (bind _newtrack_0 (Timeline|Timeline_0 PlayFromStart)
    (:Update
      (Transformation|SetActorScale3D (Variables|Default|GetInfoActor) (* (Math|Conversions|ToVector(Float) _newtrack_0) (Variables|Default|GetInfoScale))))))

(event EventAction
  (Class|BaseCharacter|OnAction))

(event EventHideUI
  (bind _newtrack_0 (Timeline|Timeline_0 ReverseFromEnd)
    (:Update
      (Transformation|SetActorScale3D (Variables|Default|GetInfoActor) (* (Math|Conversions|ToVector(Float) _newtrack_0) (Variables|Default|GetInfoScale))))))

(event EventOnNinaEndFloat
  (bind _fire (Variables|Default|GetFire))
  (bind _fire2 (Variables|Default|GetFire2))
  (bind _middlefirescale (Variables|Default|GetMiddleFireScale))
  (bind _relativescale3d (Variables|/Script/Engine.SceneComponent|GetRelativeScale3D _fire))
  (bind _relativescale3d_2 (Variables|/Script/Engine.SceneComponent|GetRelativeScale3D _fire2))
  (Components|Activation|Deactivate (Variables|Default|GetParticleSystem1))
  (Components|Activation|Deactivate (Variables|Default|GetParticleSystem))
  (CallFunction|SetMinFire)
  (bind (_direction _fireloopcurve _newtrack_2) (Timeline|FireTimeline02 Stop)
    (:Update
      (Transformation|SetRelativeScale3D _fire (Math|Vector|MakeVector (.x _relativescale3d) (.y _relativescale3d) (* _fireloopcurve _middlefirescale)))
      (Transformation|SetRelativeScale3D _fire2 (Math|Vector|MakeVector (.x _relativescale3d_2) (.y _relativescale3d_2) (* _newtrack_2 _middlefirescale))))))

(event EventEndInteraction
  (Class|InteractableBP|EndInteract(Message) (stale EventStartInteraction InteractiveActor)))

(event EventOnFixPositionEnd
  (Class|InteractableBP|FixPositionEnd(Message) (stale EventStartInteraction InteractiveActor)))

(event EventZoom
  (params (bZoom :type Boolean))
  (if (Utilities|IsValid (Variables|Default|GetGadget))
    (bind _asnina_animation_bp (CallFunction|GetAnimationBlueprint))
    (Variables|Default|SetbAimGadget true)
    (bind _output_get (Variables|/Game/Characters/Nina/Animations/Nina_Animation_BP.Nina_Animation_BP_C|SetbZoomIn _asnina_animation_bp bZoom))
    (if (and (AI|Components|NavMovement|IsFalling (Variables|Character|GetCharacterMovement)) _output_get)
      (Utilities|Time|SetGlobalTimeDilation 0.25))))

(event EventStartInteraction
  (params (InteractiveActor :type Actor%20Object%20Reference) (HitResult :type Hit%20Result%20Structure))
  (Class|InteractableBP|Interact(Message) InteractiveActor HitResult self))

(event EventBeginPlay
  (Variables|Default|SetInitialRotationRate (Variables|/Script/Engine.CharacterMovementComponent|GetRotationRate (Variables|Character|GetCharacterMovement)))
  (bind _returnvalue (Game|SpawnActorfromClass "/Game/Blueprints/Test/InfoActor.InfoActor_C" (Transformation|GetWorldTransform (Variables|Default|GetInfoSlot)) "Undefined" self 0))
  (Variables|Default|SetInfoActor _returnvalue)
  (Transformation|AttachComponentToComponent (Variables|Default|GetBackpack) (Variables|Character|GetMesh) "Back" "KeepWorld" "KeepWorld" "KeepWorld" true)
  (Development|SetHiddeninGame (Variables|Default|GetBackpack) true true)
  (CallFunction|SetMinFire)
  (bind _asbase_player_controller (Utilities|Casting|CastToBasePlayerController (Pawn|GetController)))
  (Variables|/Script/Engine.PlayerController|SetbForceFeedbackEnabled _asbase_player_controller true))

(event EventOnNinaFloat
  (bind _fire (Variables|Default|GetFire))
  (bind _fire2 (Variables|Default|GetFire2))
  (bind _fire_2 (Variables|Default|GetFire))
  (bind _fire2_2 (Variables|Default|GetFire2))
  (bind _middlefirescale (Variables|Default|GetMiddleFireScale))
  (bind _maxfirescale (Variables|Default|GetMaxFireScale))
  (bind _fire_3 (Variables|Default|GetFire))
  (bind _fire2_3 (Variables|Default|GetFire2))
  (bind _relativescale3d (Variables|/Script/Engine.SceneComponent|GetRelativeScale3D _fire))
  (bind _relativescale3d_2 (Variables|/Script/Engine.SceneComponent|GetRelativeScale3D _fire2))
  (bind _relativescale3d_3 (Variables|/Script/Engine.SceneComponent|GetRelativeScale3D _fire_2))
  (bind _relativescale3d_4 (Variables|/Script/Engine.SceneComponent|GetRelativeScale3D _fire2_2))
  (bind _relativescale3d_5 (Variables|/Script/Engine.SceneComponent|GetRelativeScale3D _fire_3))
  (bind _relativescale3d_6 (Variables|/Script/Engine.SceneComponent|GetRelativeScale3D _fire2_3))
  (Variables|/Script/Engine.CharacterMovementComponent|SetRotationRate (Variables|Character|GetCharacterMovement) (Math|Rotator|MakeRotator 0.0 0.0 (Variables|Default|GetJetpackRotationSpeed)))
  (CallFunction|FloatGate)
  (Transformation|SetRelativeScale3D _fire_2 (Math|Vector|MakeVector (.x _relativescale3d_3) (.y _relativescale3d_3) _maxfirescale))
  (Transformation|SetRelativeScale3D _fire2_2 (Math|Vector|MakeVector (.x _relativescale3d_4) (.y _relativescale3d_4) _maxfirescale))
  (Components|Activation|Activate (Variables|Default|GetParticleSystem) true)
  (Components|Activation|Activate (Variables|Default|GetParticleSystem1) true)
  (bind _newtrack_0 (Timeline|FireTimeline PlayFromStart)
    (:Update
      (Transformation|SetRelativeScale3D _fire_3 (Math|Vector|MakeVector (.x _relativescale3d_5) (.y _relativescale3d_5) (* _newtrack_0 (Variables|Default|GetMaxFireScale))))
      (Transformation|SetRelativeScale3D _fire2_3 (Math|Vector|MakeVector (.x _relativescale3d_6) (.y _relativescale3d_6) (* _newtrack_0 (Variables|Default|GetMaxFireScale))))
      (bind (_direction _fireloopcurve _newtrack_2) (Timeline|FireTimeline02 Stop)
        (:Update
          (Transformation|SetRelativeScale3D _fire (Math|Vector|MakeVector (.x _relativescale3d) (.y _relativescale3d) (* _fireloopcurve _middlefirescale)))
          (Transformation|SetRelativeScale3D _fire2 (Math|Vector|MakeVector (.x _relativescale3d_2) (.y _relativescale3d_2) (* _newtrack_2 _middlefirescale))))))
    (:Finished
      (Timeline|FireTimeline02 PlayFromStart))))

(event EventInteraction
  (Development|PrintString "Interaction")
  (Class|InteractableVolumeInterface|Interact(Message) (Variables|Default|GetInteractable)))

(event EventNinaWakeUp
  (bind _asnina_animation_bp (CallFunction|GetAnimationBlueprint))
  (Default|NinaWakeUp _asnina_animation_bp))

(fn ConstructionScript)

(fn GetAnimationBlueprint
  (bind _asnina_animation_bp (Utilities|Casting|CastToNina_Animation_BP (Components|SkeletalMesh|GetAnimInstance (Variables|Character|GetMesh))))
  (return _asnina_animation_bp))

(fn GetInteractionType
  (return "Push"))