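; Fixed-position camera actor that rotates to track the player, becoming the view target on BeginPlay if StartActive or when the player enters its trigger.
; Activation switches off FixedCameraActor_BP post-process and shadow captures, enables its own, passes the camera to BaseCharacter and leaves only this 360 camera ticking.
; Tick snaps or lerps toward the pawn.
; UpdateCaptures duplicates a per-camera render target asset when needed, then refreshes three scene captures at the camera's FOV.
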(event OnComponentBeginOverlap(CameraTrigger)
  (params (OverlappedComponent :type Primitive%20Component%20Object%20Reference) (OtherActor :type Actor%20Object%20Reference) (OtherComp :type Primitive%20Component%20Object%20Reference) (OtherBodyIndex :type Integer) (bFromSweep :type Boolean) (SweepResult :type Hit%20Result%20Structure%20%28by%20ref%29))
  (bind _returnvalue (Game|GetPlayerController 0))
  (if (== OtherActor (Game|Player|GetPlayerPawn 0))
    (Game|Player|SetViewTargetwithBlend _returnvalue self 0.0 "VTBlend_Linear" 0.0 false)
    (bind _outactors (Actor|GetAllActorsOfClass "/Game/Blueprints/FixedCameraActor_BP.FixedCameraActor_BP_C"))
    (for _array_element _outactors
      (Variables|/Script/Engine.PostProcessComponent|SetbEnabled (Variables|/Game/Blueprints/FixedCameraActor_BP.FixedCameraActor_BP_C|GetPostProcess _array_element) false)
      (Variables|/Script/Engine.SceneCaptureComponent|SetbCaptureEveryFrame (Variables|/Game/Blueprints/FixedCameraActor_BP.FixedCameraActor_BP_C|GetWithShadow _array_element) false))
    (Variables|/Script/Engine.PostProcessComponent|SetbEnabled (Variables|Default|GetPostProcess) true)
    (Variables|/Script/Engine.SceneCaptureComponent|SetbCaptureEveryFrame (Variables|Default|GetWithShadow) true)
    (bind _asbase_character (Utilities|Casting|CastToBaseCharacter (Pawn|GetControlledPawn _returnvalue)))
    (Class|BaseCharacter|SetCamera _asbase_character (Variables|CameraActor|GetCameraComponent))
    (bind _outactors_2 (Actor|GetAllActorsOfClass "360CameraActor_BP_C"))
    (for _array_element_2 _outactors_2
      (Actor|Tick|SetActorTickEnabled _array_element_2))
    (Actor|Tick|SetActorTickEnabled true)
    (Transformation|SetWorldRotation (Variables|CameraActor|GetCameraComponent) (Math|Rotator|FindLookatRotation (Transformation|GetWorldLocation (Variables|CameraActor|GetCameraComponent)) (Transformation|GetActorLocation (Game|Player|GetPlayerPawn 0))) false false)))

(event Custom|UpdateCaptures
  (bind _cameracomponent (Variables|CameraActor|GetCameraComponent))
  (bind _fieldofview (Variables|/Script/Engine.CameraComponent|GetFieldOfView _cameracomponent))
  (bind _returnvalue (Game|GetCurrentLevelName true))
  (if (Utilities|Enum|NotEqual(Enum) (Utilities|GetDisplayName (Variables|/Script/Engine.SceneCaptureComponent2D|GetTextureTarget (Variables|Default|GetNoShadow))) (Utilities|GetDisplayName self))
    (bind _returnvalue_2 (Class|AssetToolsHelpers|GetAssetTools))
    (bind _returnvalue_3 (Class|AssetTools|DuplicateAsset _returnvalue_2 (Utilities|GetDisplayName self) (Utilities|String|Append "/Game/RenderTargets/" _returnvalue "/") (Variables|Default|GetRenderTarget)))
    (bind _astexture_render_target_2d (Utilities|Casting|CastToTextureRenderTarget2D _returnvalue_3))
    (Variables|/Script/Engine.SceneCaptureComponent2D|SetTextureTarget (Variables|Default|GetNoShadow) _astexture_render_target_2d))
  (Variables|/Script/Engine.SceneCaptureComponent2D|SetFOVAngle (Variables|Default|GetExport) _fieldofview)
  (Variables|/Script/Engine.SceneCaptureComponent2D|SetFOVAngle (Variables|Default|GetWithShadow) _fieldofview)
  (Variables|/Script/Engine.SceneCaptureComponent2D|SetFOVAngle (Variables|Default|GetNoShadow) _fieldofview)
  (Rendering|SceneCapture|CaptureScene (Variables|Default|GetExport) :!class /Script/Engine.SceneCaptureComponent2D)
  (Rendering|SceneCapture|CaptureScene (Variables|Default|GetWithShadow) :!class /Script/Engine.SceneCaptureComponent2D)
  (Rendering|SceneCapture|CaptureScene (Variables|Default|GetNoShadow) :!class /Script/Engine.SceneCaptureComponent2D)
  (Development|PrintString "CapturesUpdated"))

(event Custom|ResetTriggerLocation
  (Transformation|SetWorldLocation (Variables|Default|GetCameraTrigger) (Transformation|GetActorLocation) false false))

(event EventBeginPlay
  (bind _returnvalue (Game|GetPlayerController 0))
  (if (Variables|Default|GetStartActive)
    (Game|Player|SetViewTargetwithBlend _returnvalue self 0.0 "VTBlend_Linear" 0.0 false)
    (bind _outactors (Actor|GetAllActorsOfClass "/Game/Blueprints/FixedCameraActor_BP.FixedCameraActor_BP_C"))
    (for _array_element _outactors
      (Variables|/Script/Engine.PostProcessComponent|SetbEnabled (Variables|/Game/Blueprints/FixedCameraActor_BP.FixedCameraActor_BP_C|GetPostProcess _array_element) false)
      (Variables|/Script/Engine.SceneCaptureComponent|SetbCaptureEveryFrame (Variables|/Game/Blueprints/FixedCameraActor_BP.FixedCameraActor_BP_C|GetWithShadow _array_element) false))
    (Variables|/Script/Engine.PostProcessComponent|SetbEnabled (Variables|Default|GetPostProcess) true)
    (Variables|/Script/Engine.SceneCaptureComponent|SetbCaptureEveryFrame (Variables|Default|GetWithShadow) true)
    (bind _asbase_character (Utilities|Casting|CastToBaseCharacter (Pawn|GetControlledPawn _returnvalue)))
    (Class|BaseCharacter|SetCamera _asbase_character (Variables|CameraActor|GetCameraComponent))
    (bind _outactors_2 (Actor|GetAllActorsOfClass "360CameraActor_BP_C"))
    (for _array_element_2 _outactors_2
      (Actor|Tick|SetActorTickEnabled _array_element_2))
    (Actor|Tick|SetActorTickEnabled true)
    (Transformation|SetWorldRotation (Variables|CameraActor|GetCameraComponent) (Math|Rotator|FindLookatRotation (Transformation|GetWorldLocation (Variables|CameraActor|GetCameraComponent)) (Transformation|GetActorLocation (Game|Player|GetPlayerPawn 0))) false false)))

(event Collision|EventActorBeginOverlap
  (params (OtherActor :type Actor%20Object%20Reference)))

(event EventTick
  (params (DeltaSeconds :type Float%20%28single-precision%29))
  (bind _returnvalue (Game|Player|GetPlayerPawn 0))
  (bind _cameracomponent (Variables|CameraActor|GetCameraComponent))
  (bind _returnvalue_2 (Transformation|GetWorldLocation _cameracomponent))
  (bind _returnvalue_3 (Transformation|GetActorLocation _returnvalue))
  (bind _returnvalue_4 (Math|Rotator|FindLookatRotation _returnvalue_2 _returnvalue_3))
  (if (Variables|Default|GetFollowDelay)
    (Transformation|SetWorldRotation (Variables|CameraActor|GetCameraComponent) (Math|Rotator|Lerp(Rotator) (Transformation|GetWorldRotation _cameracomponent) _returnvalue_4 (* (Variables|Default|GetFollowSpeed) DeltaSeconds) true) false false)
    (else
      (Transformation|SetWorldRotation (Variables|CameraActor|GetCameraComponent) _returnvalue_4 false false))))

(fn ConstructionScript)