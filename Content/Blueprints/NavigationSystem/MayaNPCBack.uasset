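; Maya companion NPC, likely a dog, that takes Follow, Wait, Fetch and Retrieve orders when within range of the player, Nina.
; AI MoveTo drives movement, with random wandering available, while Tick blends speed, direction and look-at into Maya_Animation_BP by state.
; Fetch attaches the target to a jaw socket, or line-traces and launches Maya toward unreached targets before retrying.
; Retrieve carries it to Nina, then waits without releasing it.
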(event Custom|SitEvent
  (params (newState :type Boolean))
  (Default|SitEvent (Variables|Default|GetAnim) newState))

(event Custom|Follow
  (bind _canacceptorders (CallFunction|RandomlyAcceptOrder))
  (if _canacceptorders
    (Variables|Default|SetDesiredDistanceToTarget 1e+02)
    (Variables|Default|SetTarget (Variables|Default|GetNina))
    (Variables|Default|SetState "NewEnumerator1")
    (CallFunction|SitEvent false)
    (AI|AIMoveTo self "0, 0, 0" (Variables|Default|GetNina) (Variables|Default|GetDesiredDistanceToTarget) false
      (:then
        (Variables|Default|SetNotMoving false))
      (:OnSuccess
        (Variables|Default|SetNotMoving true :!label _label))
      (:OnFail
        (goto _label)))))

(event Custom|Wait
  (bind _canacceptorders (CallFunction|RandomlyAcceptOrder))
  (if _canacceptorders
    (Variables|Default|SetState "NewEnumerator0")
    (CallFunction|SitEvent true)))

(event Custom|MoveNPC
  (Variables|Default|SetState "NewEnumerator4")
  (CallFunction|SitEvent false)
  (bind _output_get (Variables|Default|SetRandom%20Location (.RandomLocation (AI|Navigation|GetRandomReachablePointinRadius (Transformation|GetActorLocation) 5e+02 0 0))))
  (AI|AIMoveTo self _output_get 0 5.0 false
    (:OnSuccess
      _)
    (:OnFail
      _))
  (Utilities|FlowControl|Delay (Math|Random|RandomFloatinRange 2.0 5.0))
  (CallFunction|MoveNPC))

(event Custom|Fetch
  (bind _returnvalue (Transformation|GetActorLocation))
  (bind _returnvalue_2 (Math|Vector|VectorUp))
  (bind _returnvalue_3 (Transformation|GetActorLocation))
  (bind _canacceptorders (CallFunction|RandomlyAcceptOrder))
  (if _canacceptorders
    (if (not (Variables|Default|GetCarryingObject))
      (Variables|Default|SetTarget (Variables|Default|GetTempTarget))
      (Variables|Default|SetDesiredDistanceToTarget 25.0)
      (Variables|Default|SetState "NewEnumerator2")
      (CallFunction|SitEvent false)
      (AI|AIMoveTo self "0, 0, 0" (Variables|Default|GetTarget) (Variables|Default|GetDesiredDistanceToTarget) false :!label _label
        (:then
          (Variables|Default|SetNotMoving false))
        (:OnSuccess
          (if (<= (Math|Vector|Distance(Vector) (Transformation|GetActorLocation) (Transformation|GetActorLocation (Variables|Default|GetTarget))) (* (Variables|Default|GetDesiredDistanceToTarget) 2.0))
            (Variables|Default|SetNotMoving true)
            (Variables|/Game/Characters/Maya/Maya_Animation_BP.Maya_Animation_BP_C|SetGrab (Variables|Default|GetAnim) true)
            (Utilities|FlowControl|Delay 0.25)
            (Transformation|AttachComponentToComponent (Variables|Default|GetTarget) (Variables|Character|GetMesh) "JawSocket" "KeepRelative" "KeepRelative" "KeepRelative" true)
            (Transformation|SetActorRelativeTransform (Variables|Default|GetTarget) (Math|Transform|MakeTransform "0, 0, 0" "0.000000,0.000000,90.000000" "1.000000,1.000000,1.000000") false false)
            (Variables|Default|SetCarryingObject true)
            (Variables|/Game/Characters/Maya/Maya_Animation_BP.Maya_Animation_BP_C|SetGrab (Variables|Default|GetAnim) false)
            (CallFunction|Wait)
            (Development|PrintString "SUCCESS!" true true "(R=0.070890,G=1.000000,B=0.000000,A=1.000000)")
            (else
              (Development|PrintString (Utilities|String|ToString(Float) (Math|Vector|Distance(Vector) (Transformation|GetActorLocation) (Transformation|GetActorLocation (Variables|Default|GetTarget)))))
              (bind _outhit (Collision|LineTraceByChannel (+ (+ _returnvalue (* (Math|Vector|Normalize (- (Transformation|GetActorLocation (Variables|Default|GetTarget)) _returnvalue)) 1e+02)) (* _returnvalue_2 2e+02)) (+ (+ _returnvalue (* (Math|Vector|Normalize (- (Transformation|GetActorLocation (Variables|Default|GetTarget)) _returnvalue)) 1e+02)) (* _returnvalue_2 -2.5e+02)) "TraceTypeQuery1" false 0 "Persistent"))
              (if (> (.Z (Class|KismetMathLibrary|BreakVector3f (.impactpoint _outhit))) (.Z (Math|Vector|BreakVector _returnvalue_3)))
                (bind _outhit_2 (Collision|LineTraceByChannel _returnvalue_3 (+ _returnvalue (* (Math|Vector|Normalize (- (Transformation|GetActorLocation (Variables|Default|GetTarget)) _returnvalue)) 1e+02)) "TraceTypeQuery1" false 0 "Persistent"))
                (bind _outlaunchvelocity (Game|SuggestProjectileVelocityCustomArc (Transformation|GetActorLocation) (Math|Vector|MakeVector (.X (Class|KismetMathLibrary|BreakVector3f (.impactpoint _outhit_2))) (.Y (Class|KismetMathLibrary|BreakVector3f (.impactpoint _outhit_2))) (.Z (Class|KismetMathLibrary|BreakVector3f (.impactpoint _outhit)))) 0.0 0.5))
                (Character|LaunchCharacter (* _outlaunchvelocity 1.8) true true)
                (else
                  (Character|LaunchCharacter (* (+ (Math|Vector|VectorUp) (Transformation|GetActorForwardVector)) (Variables|Default|GetPushForce)) true true)))
              (Utilities|FlowControl|Delay 3.0)
              (goto _label))))
        (:OnFail
          (Variables|Default|SetNotMoving true)
          (CallFunction|Wait)
          (Development|PrintString "FAILED!" true true "(R=1.000000,G=0.060613,B=0.000000,A=1.000000)"))))))

(event Custom|Retrieve
  (bind _canacceptorders (CallFunction|RandomlyAcceptOrder))
  (if _canacceptorders
    (if (Variables|Default|GetCarryingObject)
      (Variables|Default|SetDesiredDistanceToTarget 1e+02)
      (Variables|Default|SetTarget (Variables|Default|GetNina))
      (Variables|Default|SetState "NewEnumerator1")
      (CallFunction|SitEvent false)
      (AI|AIMoveTo self "0, 0, 0" (Variables|Default|GetNina) (Variables|Default|GetDesiredDistanceToTarget) false
        (:then
          (Variables|Default|SetNotMoving false))
        (:OnSuccess
          (Variables|Default|SetNotMoving true :!label _label)
          (CallFunction|Wait))
        (:OnFail
          (goto _label))))))

(event EventBeginPlay
  (bind _output_get (Variables|Default|SetNina (Game|GetPlayerCharacter 0)))
  (Variables|Default|SetTarget _output_get)
  (bind _asmaya_animation_bp (Utilities|Casting|CastToMaya_Animation_BP (Components|SkeletalMesh|GetAnimInstance (Variables|Character|GetMesh))))
  (Variables|Default|SetAnim _asmaya_animation_bp))

(event EventTick
  (params (DeltaSeconds :type Float%20%28single-precision%29))
  (bind _returnvalue (Transformation|GetActorLocation))
  (bind _returnvalue_2 (Transformation|GetActorLocation))
  (bind _returnvalue_3 (Transformation|GetActorRightVector))
  (bind _returnvalue_4 (* DeltaSeconds 5.0))
  (bind _target (Variables|Default|GetTarget))
  (bind _target_2 (Variables|Default|GetTarget))
  (bind _returnvalue_5 (Transformation|GetActorLocation _target_2))
  (bind _returnvalue_6 (Transformation|GetActorLocation _target))
  (bind _returnvalue_7 (Math|Vector|Distance(Vector) _returnvalue _returnvalue_6))
  (bind _returnvalue_8 (- _returnvalue_5 _returnvalue_2))
  (bind _returnvalue_9 (Math|Vector|Normalize _returnvalue_8))
  (bind _returnvalue_10 (Math|Vector|DotProduct _returnvalue_3 _returnvalue_9))
  (bind _output_get (Variables|Default|SetTargetLocation (Math|Vector|Lerp(Vector) (Variables|Default|GetTargetLocation) (Transformation|GetActorLocation (Variables|Default|GetTarget)) DeltaSeconds)))
  (switch Utilities|FlowControl|Switch|SwitchonMayaState (Variables|Default|GetState)
    (:NewEnumerator0
      (Variables|/Game/Characters/Maya/Maya_Animation_BP.Maya_Animation_BP_C|SetLookAt (Variables|Default|GetAnim) _output_get)
      (bind _output_get_2 (Variables|Default|SetSpeed (Math|Float|Lerp (Variables|Default|GetSpeed) 0.0 (* DeltaSeconds 5.0))))
      (bind _output_get_3 (Variables|/Game/Characters/Maya/Maya_Animation_BP.Maya_Animation_BP_C|SetSpeed (Variables|Default|GetAnim) _output_get_2))
      (Variables|/Script/Engine.CharacterMovementComponent|SetMaxWalkSpeed (Variables|Character|GetCharacterMovement) _output_get_3))
    (:NewEnumerator1
      (Variables|/Game/Characters/Maya/Maya_Animation_BP.Maya_Animation_BP_C|SetLookAt (Variables|Default|GetAnim) _output_get :!label _label)
      (if (Variables|Default|GetNotMoving)
        (bind _output_get_4 (Variables|Default|SetSpeed (Math|Float|Lerp (Variables|Default|GetSpeed) 0.0 _returnvalue_4)))
        (bind _output_get_5 (Variables|/Game/Characters/Maya/Maya_Animation_BP.Maya_Animation_BP_C|SetSpeed (Variables|Default|GetAnim) _output_get_4))
        (Variables|/Script/Engine.CharacterMovementComponent|SetMaxWalkSpeed (Variables|Character|GetCharacterMovement) _output_get_5)
        (bind _output_get_6 (Variables|Default|SetDirection (Math|Float|Lerp (Variables|Default|GetDirection) 0.0 _returnvalue_4)))
        (Variables|/Game/Characters/Maya/Maya_Animation_BP.Maya_Animation_BP_C|SetDirection (Variables|Default|GetAnim) _output_get_6)
        (if (Utilities|Enum|Equal(Enum) (Variables|Default|GetState) "NewEnumerator1")
          (bind _output_get_7 (Variables|Default|SetFarToNina (> _returnvalue_7 (* (Variables|Default|GetDesiredDistanceToTarget) 2.0))))
          (if _output_get_7
            (CallFunction|Follow)))
        (else
          (bind _output_get_8 (Variables|Default|SetSpeed (Math|Float|Lerp (Variables|Default|GetSpeed) (- _returnvalue_7 (+ (Variables|Default|GetDesiredDistanceToTarget) 0.0)) DeltaSeconds)))
          (bind _output_get_9 (Variables|/Game/Characters/Maya/Maya_Animation_BP.Maya_Animation_BP_C|SetSpeed (Variables|Default|GetAnim) (* _output_get_8 (- 1.0 (* (Math|Float|Absolute(Float) _returnvalue_10) 0.75)))))
          (Variables|/Script/Engine.CharacterMovementComponent|SetMaxWalkSpeed (Variables|Character|GetCharacterMovement) _output_get_9)
          (bind _output_get_10 (Variables|Default|SetDirection _returnvalue_10))
          (Variables|/Game/Characters/Maya/Maya_Animation_BP.Maya_Animation_BP_C|SetDirection (Variables|Default|GetAnim) _output_get_10))))
    (:NewEnumerator2
      (goto _label))
    (:NewEnumerator4
      (bind _output_get_11 (Variables|Default|SetSpeed 5e+01))
      (bind _output_get_12 (Variables|/Game/Characters/Maya/Maya_Animation_BP.Maya_Animation_BP_C|SetSpeed (Variables|Default|GetAnim) _output_get_11))
      (Variables|/Script/Engine.CharacterMovementComponent|SetMaxWalkSpeed (Variables|Character|GetCharacterMovement) _output_get_12)
      (bind _output_get_13 (Variables|Default|SetDirection (Math|Vector|DotProduct (Transformation|GetActorRightVector) (Math|Vector|Normalize (- (Variables|Default|GetRandom%20Location) (Transformation|GetActorLocation))))))
      (Variables|/Game/Characters/Maya/Maya_Animation_BP.Maya_Animation_BP_C|SetDirection (Variables|Default|GetAnim) _output_get_13))))

(fn ConstructionScript)

(fn RandomlyAcceptOrder
  (if (> (Math|Random|RandomFloat) 0.0)
    (return (<= (Math|Vector|Distance(Vector) (Transformation|GetActorLocation) (Transformation|GetActorLocation (Variables|Default|GetNina))) (Variables|Default|GetOrdersMaxDistance)))))