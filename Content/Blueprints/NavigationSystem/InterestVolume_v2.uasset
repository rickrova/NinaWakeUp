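; InterestVolume_v2 is a navigation trigger volume that can distract the Maya NPC guide when she walks into it.
; On overlap it rolls a random float against Appeal, and on success disables its collision so it cannot distract her again.
; It targets the guide at RelatedItem, or itself if none is set, then stops her movement, makes her drop her item and calls Fetch.
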(event EventBeginPlay)

(event Collision|EventActorBeginOverlap
  (params (OtherActor :type Actor%20Object%20Reference))
  (bind _relateditem (Variables|Default|GetRelatedItem))
  (bind _asmaya_npcguide (Utilities|Casting|CastToMayaNPCGuide OtherActor))
  (if (<= (Math|Random|RandomFloat) (Variables|Default|GetAppeal))
    (Collision|SetCollisionEnabled (Variables|Default|GetCollisionComponent) "NoCollision")
    (if (== _relateditem 0)
      (Variables|/Game/Blueprints/NavigationSystem/MayaNPCGuide.MayaNPCGuide_C|SetTarget _asmaya_npcguide self)
      (else
        (Variables|/Game/Blueprints/NavigationSystem/MayaNPCGuide.MayaNPCGuide_C|SetTarget _asmaya_npcguide _relateditem)))
    (Components|Movement|StopMovementImmediately (Variables|/Script/Engine.Character|GetCharacterMovement _asmaya_npcguide))
    (Default|DropItem _asmaya_npcguide)
    (Default|Fetch _asmaya_npcguide)
    (Development|PrintString "Maya lost her focus" true true "(R=1.000000,G=0.000000,B=0.088870,A=1.000000)" 1e+02)))

(event EventTick
  (params (DeltaSeconds :type Float%20%28single-precision%29)))

(fn ConstructionScript)