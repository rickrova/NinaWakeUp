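; MayaNPCGuide is the navigation guide character for Maya, an NPC companion that waits, wanders, follows the player and fetches or retrieves items.
; Command events set a state, start AI moves and mirror orders to a Follower actor, while Tick drives wander timing and animation speed, direction and look-at.
; When a move ends short of its target, line traces find a landing point to teleport to, with a Follower jump for higher ledges.
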(event Custom|SitEvent
  (params (newState :type Boolean))
  (Default|SitEvent (Variables|Default|GetAnim) newState))

(event Custom|Follow
  (Variables|/Script/Engine.CharacterMovementComponent|SetMaxWalkSpeed (Variables|Character|GetCharacterMovement) 2e+02)
  (Default|Follow (Variables|Default|GetFollower))
  (Variables|Default|SetDesiredDistanceToTarget 5e+01)
  (Variables|Default|SetTarget (Variables|Default|GetNina))
  (Variables|Default|SetState "NewEnumerator1")
  (CallFunction|SitEvent false)
  (CallFunction|AIMoveto)
  (Development|PrintString "Following"))

(event Custom|Wait
  (Development|PrintString "ENTRA EL WEIT" true true "(R=1.000000,G=0.000000,B=0.191609,A=1.000000)" 1e+02)
  (Default|Wait (Variables|Default|GetFollower))
  (Variables|Default|SetState "NewEnumerator0")
  (CallFunction|SitEvent true)
  (Components|Movement|StopMovementImmediately (Variables|Character|GetCharacterMovement self))
  (Transformation|SetActorLocation (Transformation|GetActorLocation (Variables|Default|GetFollower)) false false)
  (Variables|Default|SetWanderingTimer (+ (* (Math|Random|RandomFloat) 6e+01) 6e+01)))

(event Custom|Wandering
  (Variables|/Script/Engine.CharacterMovementComponent|SetMaxWalkSpeed (Variables|Character|GetCharacterMovement) 1e+02)
  (Default|Wandering (Variables|Default|GetFollower))
  (Variables|Default|SetState "NewEnumerator4")
  (CallFunction|SitEvent false)
  (bind _output_get (Variables|Default|SetRandom%20Location (.RandomLocation (AI|Navigation|GetRandomReachablePointinRadius (Transformation|GetActorLocation) 5e+02 0 0))))
  (AI|AIMoveTo self _output_get 0 5.0 false
    (:OnSuccess
      _)
    (:OnFail
      _))
  (if (Utilities|Enum|Equal(Enum) (Variables|Default|GetState) "NewEnumerator4")
    (CallFunction|Wandering)))

(event Custom|Fetch
  (bind _target (Variables|Default|GetTarget))
  (Development|PrintString "START FETCH" true true "(R=0.000000,G=0.660000,B=1.000000,A=1.000000)" 1e+02)
  (if (and (!= _target 0) (!= _target (Game|Player|GetPlayerPawn 0)))
    (Variables|/Script/Engine.CharacterMovementComponent|SetMaxWalkSpeed (Variables|Character|GetCharacterMovement) 2e+02)
    (if (not (Variables|Default|GetCarryingObject))
      (Default|Fetch (Variables|Default|GetFollower))
      (Variables|Default|SetDesiredDistanceToTarget 25.0)
      (Variables|Default|SetState "NewEnumerator2")
      (CallFunction|SitEvent false)
      (CallFunction|AIMoveto)
      (Development|PrintString "START MOVING TO FETCH" true true "(R=0.000000,G=0.660000,B=1.000000,A=1.000000)" 1e+02))))

(event Custom|Retrieve
  (Variables|/Script/Engine.CharacterMovementComponent|SetMaxWalkSpeed (Variables|Character|GetCharacterMovement) 2e+02)
  (if (Variables|Default|GetCarryingObject)
    (Default|Retrieve (Variables|Default|GetFollower))
    (Variables|Default|SetDesiredDistanceToTarget 1e+02)
    (Variables|Default|SetTarget (Variables|Default|GetNina))
    (Variables|Default|SetState "NewEnumerator3")
    (CallFunction|SitEvent false)
    (CallFunction|AIMoveto)
    (Development|PrintString "Retrieving")))

(event Custom|AIMoveTo
  (bind _returnvalue (Transformation|GetActorLocation))
  (bind _returnvalue_2 (Transformation|GetActorLocation))
  (bind _returnvalue_3 (Transformation|GetActorLocation))
  (bind _returnvalue_4 (Math|Vector|VectorUp))
  (bind _desireddistancetotarget (Variables|Default|GetDesiredDistanceToTarget))
  (bind _target (Variables|Default|GetTarget))
  (bind _returnvalue_5 (Math|Conversions|ToVector2D(Vector) _returnvalue))
  (bind _returnvalue_6 (Transformation|GetActorLocation _target))
  (bind _returnvalue_7 (Transformation|GetActorLocation _target))
  (bind _returnvalue_8 (* _desireddistancetotarget 2.0))
  (bind _returnvalue_9 (Math|Conversions|ToVector2D(Vector) _returnvalue_6))
  (bind _returnvalue_10 (- _returnvalue_7 _returnvalue_2))
  (bind _returnvalue_11 (Math|Vector|Distance2D(Vector) _returnvalue_9 _returnvalue_5))
  (bind _returnvalue_12 (Math|Vector|Normalize _returnvalue_10))
  (bind _returnvalue_13 (* _returnvalue_12 1e+02))
  (bind _returnvalue_14 (+ _returnvalue_2 _returnvalue_13))
  (bind _movementresult (AI|AIMoveTo self "0, 0, 0" _target _desireddistancetotarget false)
    (:then
      (Variables|Default|SetNotMoving false))
    (:OnSuccess
      (Development|PrintString "siccess" true true "(R=0.000000,G=0.660000,B=1.000000,A=1.000000)" 1e+02)
      (if (<= _returnvalue_11 _returnvalue_8)
        (Variables|Default|SetNotMoving true)
        (CallFunction|EndMovingAction)
        (else
          (Development|PrintString (Utilities|String|ToString(Float) _returnvalue_11))
          (Development|PrintString "RED ALERT" true true "(R=1.000000,G=0.000000,B=0.066797,A=1.000000)")
          (Development|PrintString (Utilities|String|ToString(Float) _returnvalue_8) true true "(R=1.000000,G=0.000000,B=0.235706,A=1.000000)")
          (bind _outhit (Collision|LineTraceByChannel (+ _returnvalue_14 (* _returnvalue_4 2e+02)) (+ _returnvalue_14 (* _returnvalue_4 -2.5e+02)) "TraceTypeQuery1" false 0 "Persistent"))
          (if (> (.Z (Class|KismetMathLibrary|BreakVector3f (.impactpoint _outhit))) (.Z (Math|Vector|BreakVector _returnvalue_3)))
            (bind _outhit_2 (Collision|LineTraceByChannel _returnvalue_3 _returnvalue_14 "TraceTypeQuery1" false 0 "Persistent"))
            (Utilities|FlowControl|Delay 2.0)
            (Transformation|SetActorLocation (+ (Math|Vector|MakeVector (.X (Class|KismetMathLibrary|BreakVector3f (.impactpoint _outhit_2))) (.Y (Class|KismetMathLibrary|BreakVector3f (.impactpoint _outhit_2))) (.Z (Class|KismetMathLibrary|BreakVector3f (.impactpoint _outhit)))) "0.000000,0.000000,50.000000") false true)
            (Default|TeleportJump (Variables|Default|GetFollower) (+ (Math|Vector|MakeVector (.X (Class|KismetMathLibrary|BreakVector3f (.impactpoint _outhit_2))) (.Y (Class|KismetMathLibrary|BreakVector3f (.impactpoint _outhit_2))) (.Z (Class|KismetMathLibrary|BreakVector3f (.impactpoint _outhit)))) "0.000000,0.000000,50.000000") (Math|Rotator|MakeRotfromZX (Math|Vector|VectorUp) (* (.impactnormal _outhit_2) -1.0)))
            (Utilities|FlowControl|Delay 2.0)
            (CallFunction|AIMoveto)
            (else
              (Transformation|SetActorLocation (+ (.impactpoint _outhit) "0.000000,0.000000,50.000000") false true)
              (CallFunction|AIMoveto))))))
    (:OnFail
      (Development|PrintString "FAIOULED" true true "(R=1.000000,G=0.007345,B=0.000000,A=1.000000)" 1e+02)
      (Variables|Default|SetNotMoving true)
      (CallFunction|Wait)
      (Development|PrintString (Utilities|String|EnumtoString _movementresult) true true "(R=1.000000,G=0.060613,B=0.000000,A=1.000000)"))))

(event Custom|EndMovingAction
  (bind _state (Variables|Default|GetState))
  (Development|PrintString (Utilities|String|EnumtoString _state) true true "(R=0.717311,G=0.000000,B=1.000000,A=1.000000)" 1e+02)
  (switch Utilities|FlowControl|Switch|SwitchonMayaState _state
    (:NewEnumerator2
      (if (== (Utilities|GetClass (Variables|Default|GetTarget)) "/Game/Blueprints/Test/Item_BP.Item_BP_C")
        (Development|PrintString "START GRAB" true true "(R=0.000000,G=0.660000,B=1.000000,A=1.000000)" 1e+02)
        (Default|SetReadytoGrab (Variables|Default|GetFollower))
        (else
          (Development|PrintString "FOUND NOTHING" true true "(R=1.000000,G=0.000000,B=0.041135,A=1.000000)" 1e+02)
          (CallFunction|Wait))))
    (:NewEnumerator3
      (CallFunction|Wait)
      (Development|PrintString "will wait"))))

(event Custom|DropItem
  (Default|Drop (Variables|Default|GetFollower))
  (Variables|Default|SetCarryingObject false))

(event EventBeginPlay
  (bind _output_get (Variables|Default|SetNina (Game|GetPlayerCharacter 0)))
  (Variables|Default|SetTarget _output_get)
  (bind _asmaya_animation_bp (Utilities|Casting|CastToMaya_Animation_BP (Components|SkeletalMesh|GetAnimInstance (Variables|Character|GetMesh))))
  (Variables|Default|SetAnim _asmaya_animation_bp))

(event EventTick
  (params (DeltaSeconds :type Float%20%28single-precision%29))
  (bind _returnvalue (Transformation|GetActorLocation))
  (bind _returnvalue_2 (Transformation|GetActorLocation))
  (bind _returnvalue_3 (Transformation|GetActorRightVector))
  (bind _returnvalue_4 (* DeltaSeconds 5.0))
  (bind _target (Variables|Default|GetTarget))
  (bind _target_2 (Variables|Default|GetTarget))
  (bind _returnvalue_5 (Transformation|GetActorLocation _target_2))
  (bind _returnvalue_6 (Transformation|GetActorLocation _target))
  (bind _returnvalue_7 (Math|Vector|Distance(Vector) _returnvalue _returnvalue_6))
  (bind _returnvalue_8 (- _returnvalue_5 _returnvalue_2))
  (bind _returnvalue_9 (Math|Vector|Normalize _returnvalue_8))
  (bind _returnvalue_10 (Math|Vector|DotProduct _returnvalue_3 _returnvalue_9))
  (if (> (Variables|Default|GetWanderingTimer) 0.0)
    (bind _output_get (Variables|Default|SetWanderingTimer (- (Variables|Default|GetWanderingTimer) DeltaSeconds)))
    (if (<= _output_get 0.0)
      (if (Utilities|Enum|Equal(Enum) (Variables|Default|GetState) "NewEnumerator0")
        (CallFunction|Wandering)
        (Variables|Default|SetWanderingTimer (+ (* (Math|Random|RandomFloat) 6e+01) 6e+01) :!label _label)
        (elif (Utilities|Enum|Equal(Enum) (Variables|Default|GetState) "NewEnumerator4")
          (CallFunction|Wait)
          (goto _label)
          (else
            (Variables|Default|SetWanderingTimer 0.0))))))
  (Development|PrintString (Utilities|GetDisplayName (Variables|Default|GetTarget)) true true "(R=0.000000,G=0.660000,B=1.000000,A=1.000000)" 0.0)
  (bind _output_get_2 (Variables|Default|SetTargetLocation (Math|Vector|Lerp(Vector) (Variables|Default|GetTargetLocation) (Transformation|GetActorLocation (Variables|Default|GetTarget)) DeltaSeconds)))
  (switch Utilities|FlowControl|Switch|SwitchonMayaState (Variables|Default|GetState)
    (:NewEnumerator0
      (Variables|/Game/Characters/Maya/Maya_Animation_BP.Maya_Animation_BP_C|SetLookAt (Variables|Default|GetAnim) _output_get_2)
      (bind _output_get_3 (Variables|Default|SetSpeed (Math|Float|Lerp (Variables|Default|GetSpeed) 0.0 (* DeltaSeconds 5.0))))
      (bind _output_get_4 (Variables|/Game/Characters/Maya/Maya_Animation_BP.Maya_Animation_BP_C|SetSpeed (Variables|Default|GetAnim) _output_get_3)))
    (:NewEnumerator1
      (Variables|/Game/Characters/Maya/Maya_Animation_BP.Maya_Animation_BP_C|SetLookAt (Variables|Default|GetAnim) _output_get_2 :!label _label_2)
      (if (Variables|Default|GetNotMoving)
        (bind _output_get_5 (Variables|Default|SetSpeed (Math|Float|Lerp (Variables|Default|GetSpeed) 0.0 _returnvalue_4)))
        (bind _output_get_6 (Variables|/Game/Characters/Maya/Maya_Animation_BP.Maya_Animation_BP_C|SetSpeed (Variables|Default|GetAnim) _output_get_5))
        (bind _output_get_7 (Variables|Default|SetDirection (Math|Float|Lerp (Variables|Default|GetDirection) 0.0 _returnvalue_4)))
        (Variables|/Game/Characters/Maya/Maya_Animation_BP.Maya_Animation_BP_C|SetDirection (Variables|Default|GetAnim) _output_get_7)
        (if (Utilities|Enum|Equal(Enum) (Variables|Default|GetState) "NewEnumerator1")
          (bind _output_get_8 (Variables|Default|SetFarToNina (> _returnvalue_7 (* (Variables|Default|GetDesiredDistanceToTarget) 2.0))))
          (if _output_get_8
            (CallFunction|Follow)
            (Development|PrintString "FOLLOW NEW" true true "(R=0.000000,G=0.660000,B=1.000000,A=1.000000)" 1e+02)))
        (else
          (bind _output_get_9 (Variables|Default|SetSpeed (Math|Float|Lerp (Variables|Default|GetSpeed) (- _returnvalue_7 (+ (Variables|Default|GetDesiredDistanceToTarget) 0.0)) DeltaSeconds)))
          (bind _output_get_10 (Variables|/Game/Characters/Maya/Maya_Animation_BP.Maya_Animation_BP_C|SetSpeed (Variables|Default|GetAnim) (* _output_get_9 (- 1.0 (* (Math|Float|Absolute(Float) _returnvalue_10) 0.75)))))
          (bind _output_get_11 (Variables|Default|SetDirection _returnvalue_10))
          (Variables|/Game/Characters/Maya/Maya_Animation_BP.Maya_Animation_BP_C|SetDirection (Variables|Default|GetAnim) _output_get_11))))
    (:NewEnumerator2
      (goto _label_2))
    (:NewEnumerator4
      (bind _output_get_12 (Variables|Default|SetSpeed 0.0))
      (bind _output_get_13 (Variables|/Game/Characters/Maya/Maya_Animation_BP.Maya_Animation_BP_C|SetSpeed (Variables|Default|GetAnim) _output_get_12))
      (bind _output_get_14 (Variables|Default|SetDirection (Math|Vector|DotProduct (Transformation|GetActorRightVector) (Math|Vector|Normalize (- (Variables|Default|GetRandom%20Location) (Transformation|GetActorLocation))))))
      (Variables|/Game/Characters/Maya/Maya_Animation_BP.Maya_Animation_BP_C|SetDirection (Variables|Default|GetAnim) _output_get_14))))

(fn ConstructionScript)

(fn RandomlyAcceptOrder
  (if (> (Math|Random|RandomFloat) 0.0)
    (return (<= (Math|Vector|Distance(Vector) (Transformation|GetActorLocation) (Transformation|GetActorLocation (Variables|Default|GetNina))) (Variables|Default|GetOrdersMaxDistance)))))