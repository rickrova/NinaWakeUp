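; MayaFollower is the body of Maya, a dog-like companion that trails a Guide actor and can sit, sniff, and fetch items.
; Tick steers toward the Guide with smoothed turning and movement, then on arrival, when ready, attaches the Guide's target to JawSocket.
; Command events set pose flags and look target, which feed Maya_Animation_BP alongside speed and direction.
; TeleportJump moves the actor instantly, then eases the mesh after it as climbing.
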(event Custom|TeleportJump
  (params (NewPosition :type Vector) (NewRotation :type Rotator))
  (bind _mesh (Variables|Character|GetMesh))
  (bind _mesh_2 (Variables|Character|GetMesh))
  (Variables|Default|SetTempLocation (Transformation|GetWorldLocation _mesh))
  (Variables|Default|SetTempRotation (Transformation|GetWorldRotation _mesh))
  (Transformation|SetActorLocation NewPosition false true)
  (Transformation|SetActorRotation NewRotation)
  (Transformation|SetWorldLocation _mesh_2 (Variables|Default|GetTempLocation) false true)
  (Transformation|SetWorldRotation _mesh_2 (Variables|Default|GetTempRotation) false false)
  (Variables|Default|SetMeshOffset true)
  (Variables|/Game/Characters/Maya/Maya_Animation_BP.Maya_Animation_BP_C|SetClimbing (Variables|Default|GetAnim) true))

(event Custom|Follow
  (bind _anim (Variables|Default|GetAnim))
  (Variables|/Game/Characters/Maya/Maya_Animation_BP.Maya_Animation_BP_C|SetbSit _anim false)
  (Variables|/Game/Characters/Maya/Maya_Animation_BP.Maya_Animation_BP_C|SetbSniffing _anim false)
  (Variables|Default|SetPointTarget (Game|Player|GetPlayerPawn 0))
  (Variables|Default|SetbMoving true))

(event Custom|Fetch
  (bind _anim (Variables|Default|GetAnim))
  (Variables|/Game/Characters/Maya/Maya_Animation_BP.Maya_Animation_BP_C|SetbSit _anim false)
  (Variables|/Game/Characters/Maya/Maya_Animation_BP.Maya_Animation_BP_C|SetbSniffing _anim false)
  (Variables|Default|SetPointTarget (Variables|Default|GetGuide))
  (Variables|Default|SetbMoving true))

(event Custom|Retrieve
  (bind _anim (Variables|Default|GetAnim))
  (Variables|/Game/Characters/Maya/Maya_Animation_BP.Maya_Animation_BP_C|SetbSit _anim false)
  (Variables|/Game/Characters/Maya/Maya_Animation_BP.Maya_Animation_BP_C|SetbSniffing _anim false)
  (Variables|Default|SetPointTarget (Variables|Default|GetGuide))
  (Variables|Default|SetbMoving true))

(event Custom|Wait
  (Variables|Default|SetbMoving false)
  (Variables|Default|SetbReadyToGrab false)
  (Variables|/Game/Characters/Maya/Maya_Animation_BP.Maya_Animation_BP_C|SetbSit (Variables|Default|GetAnim) true)
  (Variables|Default|SetPointTarget (Game|Player|GetPlayerPawn 0)))

(event Custom|Wandering
  (bind _anim (Variables|Default|GetAnim))
  (Variables|/Game/Characters/Maya/Maya_Animation_BP.Maya_Animation_BP_C|SetbSit _anim false)
  (Variables|/Game/Characters/Maya/Maya_Animation_BP.Maya_Animation_BP_C|SetbSniffing _anim true)
  (Variables|Default|SetPointTarget (Variables|Default|GetGuide))
  (Variables|Default|SetbMoving true))

(event Custom|SetReadyToGrab
  (Variables|Default|SetbReadyToGrab true)
  (Development|PrintString "READY TO GRAB" true true "(R=0.000000,G=0.660000,B=1.000000,A=1.000000)" 1e+02))

(event Custom|Grab
  (bind _guide (Variables|Default|GetGuide))
  (bind _guide_2 (Variables|Default|GetGuide))
  (bind _target (Variables|/Game/Blueprints/NavigationSystem/MayaNPCGuide.MayaNPCGuide_C|GetTarget _guide_2))
  (Variables|/Game/Characters/Maya/Maya_Animation_BP.Maya_Animation_BP_C|SetGrab (Variables|Default|GetAnim) true)
  (Utilities|FlowControl|Delay 0.25)
  (bind _asitem_bp (Utilities|Casting|CastToItem_BP _target))
  (Physics|SetSimulatePhysics (Variables|/Script/NinaProject.Item|GetCollision _asitem_bp) false)
  (Transformation|AttachComponentToComponent _target (Variables|Character|GetMesh) "JawSocket" "KeepRelative" "KeepRelative" "KeepRelative" false)
  (Variables|Default|SetCarryingItem _asitem_bp)
  (Transformation|SetActorRelativeTransform _target (Math|Transform|MakeTransform "0, 0, 0" "0.000000,0.000000,90.000000" "1.000000,1.000000,1.000000") false false)
  (Variables|/Game/Blueprints/NavigationSystem/MayaNPCGuide.MayaNPCGuide_C|SetCarryingObject _guide true)
  (Variables|/Game/Characters/Maya/Maya_Animation_BP.Maya_Animation_BP_C|SetGrab (Variables|Default|GetAnim) false)
  (Default|Wait _guide)
  (Development|PrintString "RETRIEVING SUCCESS!" true true "(R=0.070890,G=1.000000,B=0.000000,A=1.000000)" 1e+02))

(event Custom|Drop
  (if (Utilities|IsValid (Variables|Default|GetCarryingItem))
    (Transformation|DetachFromActor (Variables|Default|GetCarryingItem) "KeepRelative" "KeepRelative" "KeepRelative")
    (Physics|SetSimulatePhysics (Variables|/Script/NinaProject.Item|GetCollision (Variables|Default|GetCarryingItem)) true)))

(event EventBeginPlay
  (bind _asmaya_animation_bp (Utilities|Casting|CastToMaya_Animation_BP (Components|SkeletalMesh|GetAnimInstance (Variables|Character|GetMesh))))
  (Variables|Default|SetAnim _asmaya_animation_bp)
  (Variables|Default|SetPointTarget (Game|Player|GetPlayerPawn 0)))

(event Collision|EventActorBeginOverlap
  (params (OtherActor :type Actor%20Object%20Reference)))

(event EventTick
  (params (DeltaSeconds :type Float%20%28single-precision%29))
  (bind _returnvalue (Transformation|GetActorForwardVector))
  (bind _returnvalue_2 (Transformation|GetActorLocation))
  (bind _returnvalue_3 (Transformation|GetActorLocation))
  (bind _returnvalue_4 (Transformation|GetActorRightVector))
  (bind _returnvalue_5 (* DeltaSeconds 5.0))
  (bind _guide (Variables|Default|GetGuide))
  (bind _guide_2 (Variables|Default|GetGuide))
  (bind _mesh (Variables|Character|GetMesh))
  (bind _mesh_2 (Variables|Character|GetMesh))
  (bind _returnvalue_6 (Transformation|GetActorLocation _guide))
  (bind _returnvalue_7 (Transformation|GetActorLocation _guide_2))
  (bind _relativelocation (Variables|/Script/Engine.SceneComponent|GetRelativeLocation _mesh))
  (bind _returnvalue_8 (Math|Vector|Distance(Vector) _returnvalue_2 _returnvalue_7))
  (bind _returnvalue_9 (Math|Vector|Distance(Vector) _returnvalue_3 _returnvalue_6))
  (bind _returnvalue_10 (Math|Vector|Lerp(Vector) _relativelocation "0.000000,0.000000,-48.000000" _returnvalue_5))
  (bind _returnvalue_11 (- _returnvalue_6 _returnvalue_3))
  (bind _returnvalue_12 (Math|Vector|Normalize _returnvalue_11))
  (bind _returnvalue_13 (Math|Vector|DotProduct _returnvalue_12 _returnvalue_4))
  (CallFunction|UpdateAnimation DeltaSeconds)
  (if (Variables|Default|GetMeshOffset)
    (Transformation|SetRelativeLocation _mesh _returnvalue_10 false true)
    (Transformation|SetRelativeRotation _mesh (Math|Rotator|MakeRotator 0.0 0.0 (.yaw (Math|Rotator|Lerp(Rotator) (Variables|/Script/Engine.SceneComponent|GetRelativeRotation _mesh) "0.000000,-90.000000,0.000000" (* DeltaSeconds 5.0) true))) false false)
    (if (< (Math|Vector|VectorLength _returnvalue_10) 48.1)
      (Transformation|SetRelativeLocation _mesh_2 "0.000000,0.000000,-48.000000" false true)
      (Transformation|SetRelativeRotation _mesh_2 "0.000000,-90.000000,0.000000" false false)
      (Variables|Default|SetMeshOffset false)
      (Variables|/Game/Characters/Maya/Maya_Animation_BP.Maya_Animation_BP_C|SetClimbing (Variables|Default|GetAnim) false))
    (else
      (bind _output_get (Variables|Default|SetIsInPlace (< _returnvalue_8 5.0)))
      (if _output_get
        (Development|PrintString "IN PLACE" true true "(R=0.000000,G=1.000000,B=0.110216,A=1.000000)" 0.0)
        (if (Variables|Default|GetbReadyToGrab)
          (Development|PrintString "START GRABBING" true true "(R=0.471644,G=0.000000,B=1.000000,A=1.000000)" 1e+02)
          (Variables|Default|SetbReadyToGrab false)
          (CallFunction|Grab))
        (else
          (Development|PrintString "FOLLOWING" true true "(R=0.000000,G=0.660000,B=1.000000,A=1.000000)" 0.0)
          (Development|PrintString (Utilities|String|ToString(Float) _returnvalue_8) true true "(R=0.000000,G=0.660000,B=1.000000,A=1.000000)" 0.0)
          (bind _output_get_2 (Variables|Default|SetLRot (* (Math|Float|Sign(Float) _returnvalue_13) (Math|Float|Clamp(Float) (+ (* (Math|Vector|DotProduct (Transformation|GetActorForwardVector) _returnvalue_12) -1.0) 0.1)))))
          (if (> _returnvalue_9 1e+02)
            (if (Variables|/Game/Characters/Maya/Maya_Animation_BP.Maya_Animation_BP_C|GetbAligning (Variables|Default|GetAnim))
              (Transformation|AddActorLocalRotation (Math|Rotator|MakeRotator 0.0 0.0 (Math|Float|Lerp (Variables|Default|GetLastRotationScale) (* _output_get_2 2.0) (* DeltaSeconds 1.5))) false false)
              (Variables|Default|SetLastRotationScale (Math|Float|Lerp (Variables|Default|GetLastRotationScale) (* _output_get_2 2.0) (* DeltaSeconds 1.5)))
              (Pawn|Input|AddMovementInput _returnvalue (Math|Float|Lerp (Variables|Default|GetLastMovementScale) (* _returnvalue_9 0.0) (* DeltaSeconds 1.0)) false)
              (Variables|Default|SetLastMovementScale (Math|Float|Lerp (Variables|Default|GetLastMovementScale) (* _returnvalue_9 0.0) (* DeltaSeconds 1.0)))
              (else
                (Transformation|AddActorLocalRotation (Math|Rotator|MakeRotator 0.0 0.0 (Math|Float|Lerp (Variables|Default|GetLastRotationScale) (* _returnvalue_13 2.5) (* DeltaSeconds 2.5))) false false)
                (Variables|Default|SetLastRotationScale (Math|Float|Lerp (Variables|Default|GetLastRotationScale) (* _returnvalue_13 2.5) (* DeltaSeconds 2.5)))
                (Pawn|Input|AddMovementInput _returnvalue (Math|Float|Lerp (Variables|Default|GetLastMovementScale) (* _returnvalue_9 0.0035) (* DeltaSeconds 1.0)) false)
                (Variables|Default|SetLastMovementScale (Math|Float|Lerp (Variables|Default|GetLastMovementScale) (* _returnvalue_9 0.0035) (* DeltaSeconds 1.0)))))
            (else
              (Transformation|AddActorLocalRotation (Math|Rotator|MakeRotator 0.0 0.0 (Math|Float|Lerp (Variables|Default|GetLastRotationScale) 0.0 (* DeltaSeconds 2.5))) false false)
              (bind _output_get_3 (Variables|Default|SetLastRotationScale (Math|Float|Lerp (Variables|Default|GetLastRotationScale) 0.0 (* DeltaSeconds 2.5))))
              (Variables|Default|SetLRot _output_get_3)
              (Pawn|Input|AddMovementInput _returnvalue (Math|Float|Lerp (Variables|Default|GetLastMovementScale) 0.0 (* DeltaSeconds 2.5)) false)
              (Variables|Default|SetLastMovementScale (Math|Float|Lerp (Variables|Default|GetLastMovementScale) 0.0 (* DeltaSeconds 2.5)))
              (if (< (Math|Float|Lerp (Variables|Default|GetLastMovementScale) 0.0 (* DeltaSeconds 2.5)) 0.01)
                (Development|PrintString "IN PLACE" true true "(R=0.000000,G=1.000000,B=0.110216,A=1.000000)" 0.0)
                (if (Variables|Default|GetbReadyToGrab)
                  (Development|PrintString "START GRABBING" true true "(R=0.471644,G=0.000000,B=1.000000,A=1.000000)" 1e+02)
                  (Variables|Default|SetbReadyToGrab false)
                  (CallFunction|Grab))))))))))

(fn ConstructionScript)

(fn UpdateAnimation
  (params (DeltaTime :type Float%20%28double-precision%29))
  (bind _returnvalue (Transformation|GetActorRotation))
  (bind _returnvalue_2 (Transformation|GetActorLocation))
  (bind _output_get (Variables|/Game/Characters/Maya/Maya_Animation_BP.Maya_Animation_BP_C|SetLookAt (Variables|Default|GetAnim) (Math|Vector|Lerp(Vector) (Variables|Default|GetLastLookAt) (+ (* (Transformation|GetActorForwardVector) 5e+01) (Transformation|GetActorLocation (Variables|Default|GetPointTarget))) (* DeltaTime 2.0))))
  (Variables|Default|SetLastLookAt _output_get)
  (bind _output_get_2 (Variables|/Game/Characters/Maya/Maya_Animation_BP.Maya_Animation_BP_C|SetSpeed (Variables|Default|GetAnim) (* (Math|Vector|Distance(Vector) _returnvalue_2 (Variables|Default|GetLastPosition)) 1e+02)))
  (Variables|Default|SetLastPosition _returnvalue_2)
  (Variables|Default|SetLastDirection (Math|Float|Lerp (Variables|Default|GetLastDirection) (* (.yaw (Math|Rotator|Delta(Rotator) _returnvalue (Variables|Default|GetLastRotation))) 1.0) (* DeltaTime 2.5)))
  (bind _output_get_3 (Variables|/Game/Characters/Maya/Maya_Animation_BP.Maya_Animation_BP_C|SetDirection (Variables|Default|GetAnim) (Variables|Default|GetLRot)))
  (Variables|Default|SetLastRotation _returnvalue)
  (Variables|/Game/Characters/Maya/Maya_Animation_BP.Maya_Animation_BP_C|SetbAligning (Variables|Default|GetAnim) (>= (Math|Float|Absolute(Float) _output_get_3) 0.25))
  (Variables|Default|SetTempDirection (Math|Float|Absolute(Float) _output_get_3))
  (Development|PrintString (Utilities|String|ToString(Float) _output_get_3) true true "(R=0.000000,G=0.660000,B=1.000000,A=1.000000)" 0.0)
  (if (> _output_get_2 0.0)
    _))