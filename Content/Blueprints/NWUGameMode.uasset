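; Game mode that persists the player inventory and each level's items across level changes.
; InteractionResponse asynchronously saves the inventory, then all Item_BP actors to a slot named after the level, polling each tick until done before opening the item's UnlockableLevel.
; On BeginPlay it loads both saves, refills the HUD, destroys name-matched duplicate items and respawns saved ones.
; Without an inventory save, it adds a starting notebook.
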(event Custom|OnUICreatedHandler
  (Variables|/Script/NinaProject.Inventory|SetHUD (Variables|Default|GetInventory) (stale EventBeginPlay _asnwuhud_bp)))

(event Custom|SaveGame
  (bind _inventory (Variables|Default|GetInventory))
  (Development|PrintString "SAVING" true true "(R=0.000000,G=0.660000,B=1.000000,A=1.000000)" 1e+01)
  (bind _returnvalue (SaveGame|CreateSaveGameObject "/Game/Blueprints/Inventory_Save.Inventory_Save_C"))
  (bind _output_get (Variables|Default|SetSavedGameInstance _returnvalue))
  (Variables|/Game/Blueprints/Inventory_Save.Inventory_Save_C|SetItems _output_get (Variables|/Script/NinaProject.Inventory|GetItems _inventory))
  (Variables|/Game/Blueprints/Inventory_Save.Inventory_Save_C|SetEquippedItem _output_get (Variables|/Script/NinaProject.Inventory|GetEquippedItem _inventory))
  (|AsyncSaveGametoSlot _output_get _output_get (Variables|/Game/Blueprints/Inventory_Save.Inventory_Save_C|GetSaveSlotName _output_get)
    (:Completed
      (Development|PrintString "Saved" true true "(R=0.000000,G=0.660000,B=1.000000,A=1.000000)" 1e+01)
      (bind _returnvalue_2 (SaveGame|CreateSaveGameObject "/Game/Blueprints/LevelItems_Save.LevelItems_Save_C"))
      (bind _output_get_2 (Variables|Default|SetSavedLevelItems _returnvalue_2))
      (bind _returnvalue_3 (Game|GetCurrentLevelName true))
      (Variables|/Game/Blueprints/LevelItems_Save.LevelItems_Save_C|SetSaveSlotName _output_get_2 _returnvalue_3)
      (bind _outactors (Actor|GetAllActorsOfClass "/Game/Blueprints/Test/Item_BP.Item_BP_C"))
      (for _array_element _outactors
        (Utilities|Array|Add (Variables|/Game/Blueprints/LevelItems_Save.LevelItems_Save_C|GetItems (Variables|Default|GetSavedLevelItems)) (Variables|/Script/NinaProject.Item|GetMetaData _array_element))
        (Utilities|Array|Add (Variables|/Game/Blueprints/LevelItems_Save.LevelItems_Save_C|GetTransforms (Variables|Default|GetSavedLevelItems)) (Transformation|GetActorTransform _array_element)))
      (for _array_element_2 (Variables|/Game/Blueprints/LevelItems_Save.LevelItems_Save_C|GetItems (Variables|Default|GetSavedLevelItems))
        (Development|PrintString (Utilities|String|ToString(Text) (.name _array_element_2)) true true "(R=0.000000,G=0.660000,B=1.000000,A=1.000000)" 1e+01))
      (|AsyncSaveGametoSlot (Variables|Default|GetSavedLevelItems) (Variables|/Game/Blueprints/LevelItems_Save.LevelItems_Save_C|GetSaveSlotName (Variables|Default|GetSavedLevelItems))
        (:Completed
          (Development|PrintString "ready to load" true true "(R=0.000000,G=0.660000,B=1.000000,A=1.000000)" 1e+01)
          (Variables|Default|SetbReadyToLoadLevel true))))))

(event Custom|LoadGame
  (bind _hud (Variables|Default|GetHUD))
  (bind _inventory (Variables|Default|GetInventory))
  (bind _canvascontainer (Variables|/Game/HUD/NWUHUD_BP.NWUHUD_BP_C|GetCanvasContainer _hud))
  (bind (_savegame _bsuccess) (|AsyncLoadGamefromSlot "Inventory")
    (:Completed
      (if _bsuccess
        (bind _asinventory_save (Utilities|Casting|CastToInventory_Save _savegame))
        (bind _output_get (Variables|Default|SetSavedGameInstance _asinventory_save))
        (bind _output_get_2 (Variables|/Script/NinaProject.Inventory|SetItems _inventory (Variables|/Game/Blueprints/Inventory_Save.Inventory_Save_C|GetItems _output_get)))
        (Variables|/Script/NinaProject.Inventory|SetEquippedItem _inventory (Variables|/Game/Blueprints/Inventory_Save.Inventory_Save_C|GetEquippedItem _output_get))
        (Development|PrintString "Loaded")
        (for _array_element _output_get_2
          (Default|AddItemtoInventory _canvascontainer _array_element))
        (Default|ShowEquipped _canvascontainer)
        (CallFunction|RemoveDuplicatedItems (Variables|/Script/NinaProject.Inventory|GetItems (Variables|Default|GetInventory)))
        (bind _returnvalue (Game|GetCurrentLevelName true))
        (bind (_savegame_2 _bsuccess_2) (|AsyncLoadGamefromSlot _returnvalue)
          (:Completed
            (if _bsuccess_2
              (bind _aslevel_items_save (Utilities|Casting|CastToLevelItems_Save _savegame_2))
              (bind _output_get_3 (Variables|Default|SetSavedLevelItems _aslevel_items_save))
              (CallFunction|RemoveDuplicatedItems (Variables|/Game/Blueprints/LevelItems_Save.LevelItems_Save_C|GetItems _output_get_3))
              (CallFunction|SpawnSavedItems (Variables|/Game/Blueprints/LevelItems_Save.LevelItems_Save_C|GetItems _output_get_3) (Variables|/Game/Blueprints/LevelItems_Save.LevelItems_Save_C|GetTransforms _output_get_3))
              (for _array_element_2 (Variables|Default|GetToDestroy)
                (Actor|DestroyActor _array_element_2))
              (else
                (for _array_element_3 (Variables|Default|GetToDestroy)
                  (Actor|DestroyActor _array_element_3)
                  (bind _returnvalue_2 (SaveGame|CreateSaveGameObject "/Game/Blueprints/LevelItems_Save.LevelItems_Save_C"))
                  (bind _output_get_4 (Variables|Default|SetSavedLevelItems _returnvalue_2))
                  (bind _returnvalue_3 (Game|GetCurrentLevelName true))
                  (Variables|/Game/Blueprints/LevelItems_Save.LevelItems_Save_C|SetSaveSlotName _output_get_4 _returnvalue_3)
                  (bind _outactors (Actor|GetAllActorsOfClass "/Game/Blueprints/Test/Item_BP.Item_BP_C"))
                  (for _array_element_4 _outactors
                    (Utilities|Array|Add (Variables|/Game/Blueprints/LevelItems_Save.LevelItems_Save_C|GetItems (Variables|Default|GetSavedLevelItems)) (Variables|/Script/NinaProject.Item|GetMetaData _array_element_4))
                    (Utilities|Array|Add (Variables|/Game/Blueprints/LevelItems_Save.LevelItems_Save_C|GetTransforms (Variables|Default|GetSavedLevelItems)) (Transformation|GetActorTransform _array_element_4)))
                  (|AsyncSaveGametoSlot (Variables|Default|GetSavedLevelItems) (Variables|/Game/Blueprints/LevelItems_Save.LevelItems_Save_C|GetSaveSlotName (Variables|Default|GetSavedLevelItems))))))))
        (else
          (CallFunction|AddNotebooktoInventory))))))

(event EventBeginPlay
  (bind _asnwuhud_bp (Utilities|Casting|CastToNWUHUD_BP (HUD|GetHUD (Game|GetPlayerController 0))))
  (Variables|Default|SetHUD _asnwuhud_bp)
  (EventDispatchers|BindEventtoOnUICreated _asnwuhud_bp (delegate Custom|OnUICreatedHandler))
  (Utilities|FlowControl|DelayUntilNextTick)
  (CallFunction|LoadGame))

(event EventTick
  (params (DeltaSeconds :type Float%20%28single-precision%29)))

(event EventInteractionResponse
  (params (Item :type Item%20Meta%20Structure))
  (Variables|Default|SetbReadyToLoadLevel false)
  (CallFunction|SaveGame)
  (Utilities|FlowControl|DelayUntilNextTick :!label _label)
  (if (Variables|Default|GetbReadyToLoadLevel)
    (Game|OpenLevel(byObjectReference) (.unlockablelevel Item))
    (else
      (goto _label))))

(fn ConstructionScript)

(fn AddNotebooktoInventory
  (Class|Inventory|AddtoInventory (Variables|Default|GetInventory) (LocalVariables|GetNotebook)))

(fn RemoveDuplicatedItems
  (params (InItems :type Array%20of%20Item%20Meta%20Structures))
  (bind _outactors (Actor|GetAllActorsOfClass "/Game/Blueprints/Test/Item_BP.Item_BP_C"))
  (for _array_element _outactors
    (for _array_element_2 InItems
      (if (Utilities|Enum|Equal(Enum) (.name _array_element_2) (.name (Variables|/Script/NinaProject.Item|GetMetaData _array_element)))
        (Utilities|Array|AddUnique (Variables|Default|GetToDestroy) _array_element)))))

(fn SpawnSavedItems
  (params (InItems :type Array%20of%20Item%20Meta%20Structures) (InTransforms :type Array%20of%20Transforms))
  (for (_array_element _array_index) InItems
    (bind _returnvalue (Game|SpawnActorfromClass "/Game/Blueprints/Test/Item_BP.Item_BP_C" (Utilities|Array|Get(acopy) InTransforms _array_index) "Undefined" 0 0))
    (bind _output_get (Variables|/Script/NinaProject.Item|SetMetaData _returnvalue _array_element))
    (Components|StaticMesh|SetStaticMesh (Variables|/Script/NinaProject.Item|GetVisibleComponent _returnvalue) (.staticmesh _output_get))))