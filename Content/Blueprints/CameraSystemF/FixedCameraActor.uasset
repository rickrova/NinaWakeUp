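; Fixed camera actor that switches the player's view to itself when the player pawn enters its trigger, or optionally through an interact-driven zoom.
; SetThisCamera blends the view, disables the game mode's current camera, registers itself and passes its camera to the character.
; Only the active camera keeps post process and per-frame scene capture on.
; In interaction mode, UI prompts show and Interact toggles zoom, locking movement and restoring the previous camera.
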(event OnComponentBeginOverlap(CameraTrigger)
  (params (OverlappedComponent :type Primitive%20Component%20Object%20Reference) (OtherActor :type Actor%20Object%20Reference) (OtherComp :type Primitive%20Component%20Object%20Reference) (OtherBodyIndex :type Integer) (bFromSweep :type Boolean) (SweepResult :type Hit%20Result%20Structure%20%28by%20ref%29))
  (bind _returnvalue (Game|Player|GetPlayerPawn 0))
  (if (== OtherActor _returnvalue)
    (bind _asnina_character_bp (Utilities|Casting|CastToNinaCharacter_BP _returnvalue))
    (if (and (!= (Variables|/Script/NinaProject.BaseCharacter|GetCurrentCamera _asnina_character_bp) (Variables|CameraActor|GetCameraComponent)) (!= (Variables|/Script/NinaProject.BaseCharacter|GetPendingCamera _asnina_character_bp) (Variables|CameraActor|GetCameraComponent)))
      (if (Variables|Default|GetbRequireUserInteraction)
        (Variables|/Game/Characters/Nina/NinaCharacter_BP.NinaCharacter_BP_C|SetInteractable _asnina_character_bp self)
        (Default|ShowZoominPrompt (Variables|Default|GetUI))
        (Variables|Default|SetbCanInteract true)
        (else
          (CallFunction|SetThisCamera))))))

(event OnComponentEndOverlap(CameraTrigger)
  (params (OverlappedComponent :type Primitive%20Component%20Object%20Reference) (OtherActor :type Actor%20Object%20Reference) (OtherComp :type Primitive%20Component%20Object%20Reference) (OtherBodyIndex :type Integer))
  (if (Variables|Default|GetbRequireUserInteraction)
    (Default|HideZoominPrompt (Variables|Default|GetUI))
    (Variables|Default|SetbCanInteract false)))

(event Custom|UpdateCaptures
  (Development|PrintString "send to child"))

(event Custom|OnCreateUIHandrer
  (Variables|Default|SetUI (Variables|/Game/Blueprints/NWUGameMode.NWUGameMode_C|GetWidgo (stale EventBeginPlay _asnwugame_mode))))

(event Custom|SetThisCamera
  (bind _returnvalue (Game|GetPlayerController 0))
  (Game|Player|SetViewTargetwithBlend _returnvalue self 0.0 "VTBlend_Linear" 0.0 false)
  (bind _asnwugame_mode (Utilities|Casting|CastToNWUGameMode (Game|GetGameMode)))
  (if (!= (Variables|/Game/Blueprints/NWUGameMode.NWUGameMode_C|GetCurrentCamera _asnwugame_mode) 0)
    (CallFunction|DisableThisCamera (Variables|/Game/Blueprints/NWUGameMode.NWUGameMode_C|GetCurrentCamera _asnwugame_mode)))
  (Variables|/Game/Blueprints/NWUGameMode.NWUGameMode_C|SetCurrentCamera _asnwugame_mode self)
  (Variables|/Script/Engine.PostProcessComponent|SetbEnabled (Variables|Default|GetPostProcess) true)
  (Variables|/Script/Engine.SceneCaptureComponent|SetbCaptureEveryFrame (Variables|Default|GetWithShadow) true)
  (bind _asbase_character (Utilities|Casting|CastToBaseCharacter (Pawn|GetControlledPawn _returnvalue)))
  (Class|BaseCharacter|SetCamera _asbase_character (Variables|CameraActor|GetCameraComponent)))

(event Custom|ResetTriggerLocation
  (Transformation|SetWorldLocation (Variables|Default|GetCameraTrigger) (Transformation|GetActorLocation) false false))

(event Custom|DisableThisCamera
  (Variables|/Script/Engine.PostProcessComponent|SetbEnabled (Variables|Default|GetPostProcess) false)
  (Variables|/Script/Engine.SceneCaptureComponent|SetbCaptureEveryFrame (Variables|Default|GetWithShadow) false))

(event EventBeginPlay
  (if (Variables|Default|GetbRequireUserInteraction)
    (bind _asnwugame_mode (Utilities|Casting|CastToNWUGameMode (Game|GetGameMode)))
    (EventDispatchers|BindEventtoOnCreateUI _asnwugame_mode (delegate Custom|OnCreateUIHandrer)))
  (if (Variables|Default|GetStartActive)
    (CallFunction|SetThisCamera)
    (Development|PrintString "FixedCameraMessage")))

(event Collision|EventActorBeginOverlap
  (params (OtherActor :type Actor%20Object%20Reference)))

(event EventTick
  (params (DeltaSeconds :type Float%20%28single-precision%29)))

(event EventInteract
  (bind _ui (Variables|Default|GetUI))
  (bind _ui_2 (Variables|Default|GetUI))
  (if (Variables|Default|GetbCanInteract)
    (if (Variables|Default|GetbExitThisCamera)
      (CallFunction|SetThisCamera (Variables|Default|GetPreviousCamera))
      (Default|ShowZoominPrompt _ui)
      (Default|HideZoomOutPrompt _ui)
      (bind _output_get (Variables|Default|SetbExitThisCamera false))
      (Input|SetIgnoreMoveInput (Game|GetPlayerController (Game|GetPlayerState 0)) _output_get)
      (else
        (bind _asnwugame_mode (Utilities|Casting|CastToNWUGameMode (Game|GetGameMode)))
        (Variables|Default|SetPreviousCamera (Variables|/Game/Blueprints/NWUGameMode.NWUGameMode_C|GetCurrentCamera _asnwugame_mode))
        (CallFunction|SetThisCamera)
        (Default|HideZoominPrompt _ui_2)
        (Default|ShowZoomOutPrompt _ui_2)
        (bind _output_get_2 (Variables|Default|SetbExitThisCamera true))
        (Input|SetIgnoreMoveInput (Game|GetPlayerController (Game|GetPlayerState 0)) _output_get_2)))))

(fn ConstructionScript)