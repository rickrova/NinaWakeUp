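; 360 camera actor that becomes the player's view and rotates to track the pawn, optionally with smoothed lag.
; Its trigger activates it on overlap or after a zoom-in prompt and Interact press; it can also start active.
; Activation disables other static and 360 cameras' post-process and scene captures, then enables its own.
; It also registers with the character and applies its material to the background sphere found at construction.
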(event OnComponentBeginOverlap(CameraTrigger)
  (params (OverlappedComponent :type Primitive%20Component%20Object%20Reference) (OtherActor :type Actor%20Object%20Reference) (OtherComp :type Primitive%20Component%20Object%20Reference) (OtherBodyIndex :type Integer) (bFromSweep :type Boolean) (SweepResult :type Hit%20Result%20Structure%20%28by%20ref%29))
  (bind _returnvalue (Game|Player|GetPlayerPawn 0))
  (if (== OtherActor _returnvalue)
    (bind _asnina_character_bp (Utilities|Casting|CastToNinaCharacter_BP _returnvalue))
    (if (and (!= (Variables|/Script/NinaProject.BaseCharacter|GetCurrentCamera _asnina_character_bp) (Variables|CameraActor|GetCameraComponent)) (!= (Variables|/Script/NinaProject.BaseCharacter|GetPendingCamera _asnina_character_bp) (Variables|CameraActor|GetCameraComponent)))
      (if (Variables|Default|GetbRequireUserInteraction)
        (Default|ShowZoominPrompt (Variables|Default|GetUI))
        (Variables|Default|SetbCanInteract true)
        (else
          (CallFunction|SetThisCamera))))))

(event OnComponentEndOverlap(CameraTrigger)
  (params (OverlappedComponent :type Primitive%20Component%20Object%20Reference) (OtherActor :type Actor%20Object%20Reference) (OtherComp :type Primitive%20Component%20Object%20Reference) (OtherBodyIndex :type Integer))
  (if (Variables|Default|GetbRequireUserInteraction)
    (Default|HideZoominPrompt (Variables|Default|GetUI))
    (Variables|Default|SetbCanInteract false)))

(event Custom|UpdateCaptures
  (Variables|/Script/Engine.SceneCaptureComponent|SetbCaptureEveryFrame (Variables|Default|GetExport) true))

(event Custom|OnCreateUIHandrer
  (Variables|Default|SetUI (Variables|/Game/Blueprints/NWUGameMode.NWUGameMode_C|GetWidgo (stale EventBeginPlay _asnwugame_mode))))

(event Custom|ResetTriggerLocation
  (Transformation|SetWorldLocation (Variables|Default|GetCameraTrigger) (Transformation|GetActorLocation) false false))

(event Custom|SetThisCamera
  (bind _returnvalue (Game|GetPlayerController 0))
  (Game|Player|SetViewTargetwithBlend _returnvalue self 0.0 "VTBlend_Linear" 0.0 false)
  (bind _outactors (Actor|GetAllActorsOfClass "/Game/Blueprints/CameraSystemF/StaticCameraActor_BP.StaticCameraActor_BP_C"))
  (for _array_element _outactors
    (Variables|/Script/Engine.PostProcessComponent|SetbEnabled (Variables|/Game/Blueprints/CameraSystemF/StaticCameraActor_BP.StaticCameraActor_BP_C|GetPostProcess _array_element) false)
    (Variables|/Script/Engine.SceneCaptureComponent|SetbCaptureEveryFrame (Variables|/Game/Blueprints/CameraSystemF/StaticCameraActor_BP.StaticCameraActor_BP_C|GetWithShadow _array_element) false))
  (bind _outactors_2 (Actor|GetAllActorsOfClass "/Game/Blueprints/CameraSystemF/360CameraActor_BP.360CameraActor_BP_C"))
  (for _array_element_2 _outactors_2
    (Actor|Tick|SetActorTickEnabled _array_element_2)
    (Variables|/Script/Engine.PostProcessComponent|SetbEnabled (Variables|/Game/Blueprints/CameraSystemF/360CameraActor_BP.360CameraActor_BP_C|GetPostProcess _array_element_2) false)
    (Variables|/Script/Engine.SceneCaptureComponent|SetbCaptureEveryFrame (Variables|/Game/Blueprints/CameraSystemF/360CameraActor_BP.360CameraActor_BP_C|GetWithShadow _array_element_2) false)
    (Variables|/Script/Engine.SceneCaptureComponent|SetbCaptureEveryFrame (Variables|/Game/Blueprints/CameraSystemF/360CameraActor_BP.360CameraActor_BP_C|GetNoShadow _array_element_2) false)
    (Variables|/Script/Engine.SceneCaptureComponent|SetbCaptureEveryFrame (Variables|/Game/Blueprints/CameraSystemF/360CameraActor_BP.360CameraActor_BP_C|GetBackground _array_element_2) false))
  (Variables|/Script/Engine.PostProcessComponent|SetbEnabled (Variables|Default|GetPostProcess) true)
  (Variables|/Script/Engine.SceneCaptureComponent|SetbCaptureEveryFrame (Variables|Default|GetWithShadow) true)
  (Variables|/Script/Engine.SceneCaptureComponent|SetbCaptureEveryFrame (Variables|Default|GetNoShadow) true)
  (Variables|/Script/Engine.SceneCaptureComponent|SetbCaptureEveryFrame (Variables|Default|GetBackground) true)
  (bind _asbase_character (Utilities|Casting|CastToBaseCharacter (Pawn|GetControlledPawn _returnvalue)))
  (Class|BaseCharacter|SetCamera _asbase_character (Variables|CameraActor|GetCameraComponent))
  (Actor|Tick|SetActorTickEnabled true)
  (Transformation|SetWorldRotation (Variables|CameraActor|GetCameraComponent) (Math|Rotator|FindLookatRotation (Transformation|GetWorldLocation (Variables|CameraActor|GetCameraComponent)) (Transformation|GetActorLocation (Game|Player|GetPlayerPawn 0))) false false)
  (Rendering|Material|SetMaterial (Variables|/Script/Engine.StaticMeshActor|GetStaticMeshComponent (Variables|Default|GetSphereBack)) 0 (Variables|Default|GetSphereMaterial)))

(event EventBeginPlay
  (if (Variables|Default|GetbRequireUserInteraction)
    (bind _asnwugame_mode (Utilities|Casting|CastToNWUGameMode (Game|GetGameMode)))
    (EventDispatchers|BindEventtoOnCreateUI _asnwugame_mode (delegate Custom|OnCreateUIHandrer)))
  (if (Variables|Default|GetStartActive)
    (CallFunction|SetThisCamera)))

(event Collision|EventActorBeginOverlap
  (params (OtherActor :type Actor%20Object%20Reference)))

(event EventTick
  (params (DeltaSeconds :type Float%20%28single-precision%29))
  (bind _returnvalue (Game|Player|GetPlayerPawn 0))
  (bind _cameracomponent (Variables|CameraActor|GetCameraComponent))
  (bind _returnvalue_2 (Transformation|GetWorldLocation _cameracomponent))
  (bind _returnvalue_3 (Transformation|GetActorLocation _returnvalue))
  (bind _returnvalue_4 (Math|Rotator|FindLookatRotation _returnvalue_2 _returnvalue_3))
  (if (Variables|Default|GetFollowDelay)
    (Transformation|SetWorldRotation (Variables|CameraActor|GetCameraComponent) (Math|Rotator|Lerp(Rotator) (Transformation|GetWorldRotation _cameracomponent) _returnvalue_4 (* (Variables|Default|GetFollowSpeed) DeltaSeconds) true) false false)
    (else
      (Transformation|SetWorldRotation (Variables|CameraActor|GetCameraComponent) _returnvalue_4 false false))))

(event Input|ActionEvents|InputActionInteract
  (params (Key :type Key%20Structure))
  (:Pressed
    (if (Variables|Default|GetbCanInteract)
      (CallFunction|SetThisCamera)
      (Default|HideZoominPrompt (Variables|Default|GetUI))
      (Variables|Default|SetbCanInteract false))))

(fn ConstructionScript
  (bind _outactors (Actor|GetAllActorsOfClass "/Game/Blueprints/CameraSystemF/360BackgroundSphere_BP.360BackgroundSphere_BP_C"))
  (if (> (Utilities|Array|Length _outactors) 0)
    (Variables|Default|SetSphereBack (Utilities|Array|Get(acopy) _outactors))
    (Variables|/Script/Engine.SceneCaptureComponent|SetShowOnlyActors (Variables|Default|GetBackground) (Utilities|Array|MakeArray (Utilities|Array|Get(acopy) _outactors)))))