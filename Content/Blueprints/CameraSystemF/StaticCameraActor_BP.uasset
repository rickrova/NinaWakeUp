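; Static camera actor that pairs a CameraComponent with three scene captures: NoShadow, WithShadow and Export.
; UpdateCaptures matches all three captures to the camera's FOV and enables capture every frame.
; If NoShadow's render target name differs from the actor's, it first uses editor AssetTools to duplicate a template target under /Game/RenderTargets/<level>/, named after the actor, and assigns it to NoShadow only.
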(event Collision|EventActorBeginOverlap
  (params (OtherActor :type Actor%20Object%20Reference)))

(event EventTick
  (params (DeltaSeconds :type Float%20%28single-precision%29)))

(event EventUpdateCaptures
  (bind _cameracomponent (Variables|Default|GetCameraComponent))
  (bind _fieldofview (Variables|/Script/Engine.CameraComponent|GetFieldOfView _cameracomponent))
  (bind _returnvalue (Game|GetCurrentLevelName true))
  (if (Utilities|Enum|NotEqual(Enum) (Utilities|GetDisplayName (Variables|/Script/Engine.SceneCaptureComponent2D|GetTextureTarget (Variables|Default|GetNoShadow))) (Utilities|GetDisplayName self))
    (bind _returnvalue_2 (Class|AssetToolsHelpers|GetAssetTools))
    (bind _returnvalue_3 (Class|AssetTools|DuplicateAsset _returnvalue_2 (Utilities|GetDisplayName self) (Utilities|String|Append "/Game/RenderTargets/" _returnvalue "/") (Variables|Default|GetRenderTarget)))
    (bind _astexture_render_target_2d (Utilities|Casting|CastToTextureRenderTarget2D _returnvalue_3))
    (Variables|/Script/Engine.SceneCaptureComponent2D|SetTextureTarget (Variables|Default|GetNoShadow) _astexture_render_target_2d))
  (Variables|/Script/Engine.SceneCaptureComponent2D|SetFOVAngle (Variables|Default|GetExport) _fieldofview)
  (Variables|/Script/Engine.SceneCaptureComponent2D|SetFOVAngle (Variables|Default|GetWithShadow) _fieldofview)
  (Variables|/Script/Engine.SceneCaptureComponent2D|SetFOVAngle (Variables|Default|GetNoShadow) _fieldofview)
  (Variables|/Script/Engine.SceneCaptureComponent|SetbCaptureEveryFrame (Variables|Default|GetExport) true)
  (Variables|/Script/Engine.SceneCaptureComponent|SetbCaptureEveryFrame (Variables|Default|GetWithShadow) true)
  (Variables|/Script/Engine.SceneCaptureComponent|SetbCaptureEveryFrame (Variables|Default|GetNoShadow) true))

(fn ConstructionScript)