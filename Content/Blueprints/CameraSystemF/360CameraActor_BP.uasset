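; 360CameraActor_BP is a switchable camera actor that rotates to track the player pawn, either instantly or with a smoothed follow.
; Activating it enables tick and its NoShadow and Background scene captures and applies its material to the background sphere; deactivating it stops tick and both captures.
; The construction script finds that sphere and makes it Background's show-only actor.
; UpdateCaptures leaves only this camera's Export capture running every frame.
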(event Collision|EventActorBeginOverlap
  (params (OtherActor :type Actor%20Object%20Reference)))

(event EventTick
  (params (DeltaSeconds :type Float%20%28single-precision%29))
  (bind _returnvalue (Game|Player|GetPlayerPawn 0))
  (bind _cameracomponent (Variables|Default|GetCameraComponent))
  (bind _returnvalue_2 (Transformation|GetWorldLocation _cameracomponent))
  (bind _returnvalue_3 (Transformation|GetActorLocation _returnvalue))
  (bind _returnvalue_4 (Math|Rotator|FindLookatRotation _returnvalue_2 _returnvalue_3))
  (if (Variables|Default|GetFollowDelay)
    (Transformation|SetWorldRotation (Variables|Default|GetCameraComponent) (Math|Rotator|Lerp(Rotator) (Transformation|GetWorldRotation _cameracomponent) _returnvalue_4 (* (Variables|Default|GetFollowSpeed) DeltaSeconds) true) false false)
    (else
      (Transformation|SetWorldRotation (Variables|Default|GetCameraComponent) _returnvalue_4 false false))))

(event EventDisableThisCamera
  (|CallParentFunction)
  (Actor|Tick|SetActorTickEnabled false)
  (Variables|/Script/Engine.SceneCaptureComponent|SetbCaptureEveryFrame (Variables|Default|GetNoShadow) false)
  (Variables|/Script/Engine.SceneCaptureComponent|SetbCaptureEveryFrame (Variables|Default|GetBackground) false))

(event EventSetThisCamera
  (|CallParentFunction)
  (Variables|/Script/Engine.SceneCaptureComponent|SetbCaptureEveryFrame (Variables|Default|GetNoShadow) true)
  (Variables|/Script/Engine.SceneCaptureComponent|SetbCaptureEveryFrame (Variables|Default|GetBackground) true)
  (Actor|Tick|SetActorTickEnabled true)
  (Transformation|SetWorldRotation (Variables|Default|GetCameraComponent) (Math|Rotator|FindLookatRotation (Transformation|GetWorldLocation (Variables|Default|GetCameraComponent)) (Transformation|GetActorLocation (Game|Player|GetPlayerPawn 0))) false false)
  (Rendering|Material|SetMaterial (Variables|/Script/Engine.StaticMeshActor|GetStaticMeshComponent (Variables|Default|GetSphereBack)) 0 (Variables|Default|GetSphereMaterial)))

(event EventUpdateCaptures
  (bind _outactors (Actor|GetAllActorsOfClass "360CameraActor_BP_C"))
  (for _array_element _outactors
    (Variables|/Script/Engine.SceneCaptureComponent|SetbCaptureEveryFrame (Variables|360CameraActor_BP_C|GetExport _array_element) false))
  (Variables|/Script/Engine.SceneCaptureComponent|SetbCaptureEveryFrame (Variables|Default|GetExport) true))

(fn ConstructionScript
  (bind _outactors (Actor|GetAllActorsOfClass "/Game/Blueprints/CameraSystemF/360BackgroundSphere_BP.360BackgroundSphere_BP_C"))
  (if (> (Utilities|Array|Length _outactors) 0)
    (Variables|Default|SetSphereBack (Utilities|Array|Get(acopy) _outactors))
    (Variables|/Script/Engine.SceneCaptureComponent|SetShowOnlyActors (Variables|Default|GetBackground) (Utilities|Array|MakeArray (Utilities|Array|Get(acopy) _outactors)))))