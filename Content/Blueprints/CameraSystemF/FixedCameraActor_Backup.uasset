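; Fixed camera actor that becomes the player's view on start, on trigger overlap, or through a prompted zoom interaction.
; SetThisCamera switches view target, disables post-process and captures on other static and 360 cameras, then updates character and game mode.
; Interact toggles zoom, locking movement and restoring the previous camera on exit.
; UpdateCaptures duplicates a per-camera render target asset into the level's folder and syncs scene capture FOVs to the camera.
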(event OnComponentBeginOverlap(CameraTrigger)
  (params (OverlappedComponent :type Primitive%20Component%20Object%20Reference) (OtherActor :type Actor%20Object%20Reference) (OtherComp :type Primitive%20Component%20Object%20Reference) (OtherBodyIndex :type Integer) (bFromSweep :type Boolean) (SweepResult :type Hit%20Result%20Structure%20%28by%20ref%29))
  (bind _returnvalue (Game|Player|GetPlayerPawn 0))
  (if (== OtherActor _returnvalue)
    (bind _asnina_character_bp (Utilities|Casting|CastToNinaCharacter_BP _returnvalue))
    (if (and (!= (Variables|/Script/NinaProject.BaseCharacter|GetCurrentCamera _asnina_character_bp) (Variables|CameraActor|GetCameraComponent)) (!= (Variables|/Script/NinaProject.BaseCharacter|GetPendingCamera _asnina_character_bp) (Variables|CameraActor|GetCameraComponent)))
      (if (Variables|Default|GetbRequireUserInteraction)
        (Variables|/Game/Characters/Nina/NinaCharacter_BP.NinaCharacter_BP_C|SetInteractable _asnina_character_bp self)
        (Default|ShowZoominPrompt (Variables|Default|GetUI))
        (Variables|Default|SetbCanInteract true)
        (else
          (CallFunction|SetThisCamera))))))

(event OnComponentEndOverlap(CameraTrigger)
  (params (OverlappedComponent :type Primitive%20Component%20Object%20Reference) (OtherActor :type Actor%20Object%20Reference) (OtherComp :type Primitive%20Component%20Object%20Reference) (OtherBodyIndex :type Integer))
  (if (Variables|Default|GetbRequireUserInteraction)
    (Default|HideZoominPrompt (Variables|Default|GetUI))
    (Variables|Default|SetbCanInteract false)))

(event Custom|UpdateCaptures
  (bind _cameracomponent (Variables|CameraActor|GetCameraComponent))
  (bind _fieldofview (Variables|/Script/Engine.CameraComponent|GetFieldOfView _cameracomponent))
  (bind _returnvalue (Game|GetCurrentLevelName true))
  (if (Utilities|Enum|NotEqual(Enum) (Utilities|GetDisplayName (Variables|/Script/Engine.SceneCaptureComponent2D|GetTextureTarget (Variables|Default|GetNoShadow))) (Utilities|GetDisplayName self))
    (bind _returnvalue_2 (Class|AssetToolsHelpers|GetAssetTools))
    (bind _returnvalue_3 (Class|AssetTools|DuplicateAsset _returnvalue_2 (Utilities|GetDisplayName self) (Utilities|String|Append "/Game/RenderTargets/" _returnvalue "/") (Variables|Default|GetRenderTarget)))
    (bind _astexture_render_target_2d (Utilities|Casting|CastToTextureRenderTarget2D _returnvalue_3))
    (Variables|/Script/Engine.SceneCaptureComponent2D|SetTextureTarget (Variables|Default|GetNoShadow) _astexture_render_target_2d))
  (Variables|/Script/Engine.SceneCaptureComponent2D|SetFOVAngle (Variables|Default|GetExport) _fieldofview)
  (Variables|/Script/Engine.SceneCaptureComponent2D|SetFOVAngle (Variables|Default|GetWithShadow) _fieldofview)
  (Variables|/Script/Engine.SceneCaptureComponent2D|SetFOVAngle (Variables|Default|GetNoShadow) _fieldofview)
  (Variables|/Script/Engine.SceneCaptureComponent|SetbCaptureEveryFrame (Variables|Default|GetExport) true)
  (Variables|/Script/Engine.SceneCaptureComponent|SetbCaptureEveryFrame (Variables|Default|GetWithShadow) true)
  (Variables|/Script/Engine.SceneCaptureComponent|SetbCaptureEveryFrame (Variables|Default|GetNoShadow) true))

(event Custom|OnCreateUIHandrer
  (Variables|Default|SetUI (Variables|/Game/Blueprints/NWUGameMode.NWUGameMode_C|GetWidgo (stale EventBeginPlay _asnwugame_mode))))

(event Custom|SetThisCamera
  (bind _returnvalue (Game|GetPlayerController 0))
  (Game|Player|SetViewTargetwithBlend _returnvalue self 0.0 "VTBlend_Linear" 0.0 false)
  (bind _outactors (Actor|GetAllActorsOfClass "/Game/Blueprints/CameraSystemF/StaticCameraActor_BP.StaticCameraActor_BP_C"))
  (for _array_element _outactors
    (Variables|/Script/Engine.PostProcessComponent|SetbEnabled (Variables|/Game/Blueprints/CameraSystemF/StaticCameraActor_BP.StaticCameraActor_BP_C|GetPostProcess _array_element) false)
    (Variables|/Script/Engine.SceneCaptureComponent|SetbCaptureEveryFrame (Variables|/Game/Blueprints/CameraSystemF/StaticCameraActor_BP.StaticCameraActor_BP_C|GetWithShadow _array_element) false))
  (bind _outactors_2 (Actor|GetAllActorsOfClass "/Game/Blueprints/CameraSystemF/360CameraActor_BP.360CameraActor_BP_C"))
  (for _array_element_2 _outactors_2
    (Actor|Tick|SetActorTickEnabled _array_element_2)
    (Variables|/Script/Engine.PostProcessComponent|SetbEnabled (Variables|/Game/Blueprints/CameraSystemF/360CameraActor_BP.360CameraActor_BP_C|GetPostProcess _array_element_2) false)
    (Variables|/Script/Engine.SceneCaptureComponent|SetbCaptureEveryFrame (Variables|/Game/Blueprints/CameraSystemF/360CameraActor_BP.360CameraActor_BP_C|GetWithShadow _array_element_2) false)
    (Variables|/Script/Engine.SceneCaptureComponent|SetbCaptureEveryFrame (Variables|/Game/Blueprints/CameraSystemF/360CameraActor_BP.360CameraActor_BP_C|GetNoShadow _array_element_2) false)
    (Variables|/Script/Engine.SceneCaptureComponent|SetbCaptureEveryFrame (Variables|/Game/Blueprints/CameraSystemF/360CameraActor_BP.360CameraActor_BP_C|GetBackground _array_element_2) false))
  (Variables|/Script/Engine.PostProcessComponent|SetbEnabled (Variables|Default|GetPostProcess) true)
  (Variables|/Script/Engine.SceneCaptureComponent|SetbCaptureEveryFrame (Variables|Default|GetWithShadow) true)
  (bind _asbase_character (Utilities|Casting|CastToBaseCharacter (Pawn|GetControlledPawn _returnvalue)))
  (Class|BaseCharacter|SetCamera _asbase_character (Variables|CameraActor|GetCameraComponent))
  (bind _asnwugame_mode (Utilities|Casting|CastToNWUGameMode (Game|GetGameMode)))
  (Variables|/Game/Blueprints/NWUGameMode.NWUGameMode_C|SetCurrentCamera _asnwugame_mode self))

(event Custom|ResetTriggerLocation
  (Transformation|SetWorldLocation (Variables|Default|GetCameraTrigger) (Transformation|GetActorLocation) false false))

(event EventBeginPlay
  (if (Variables|Default|GetbRequireUserInteraction)
    (bind _asnwugame_mode (Utilities|Casting|CastToNWUGameMode (Game|GetGameMode)))
    (EventDispatchers|BindEventtoOnCreateUI _asnwugame_mode (delegate Custom|OnCreateUIHandrer)))
  (if (Variables|Default|GetStartActive)
    (CallFunction|SetThisCamera)))

(event Collision|EventActorBeginOverlap
  (params (OtherActor :type Actor%20Object%20Reference)))

(event EventTick
  (params (DeltaSeconds :type Float%20%28single-precision%29)))

(event EventInteract
  (bind _ui (Variables|Default|GetUI))
  (bind _ui_2 (Variables|Default|GetUI))
  (if (Variables|Default|GetbCanInteract)
    (if (Variables|Default|GetbExitThisCamera)
      (CallFunction|SetThisCamera (Variables|Default|GetPreviousCamera))
      (Default|ShowZoominPrompt _ui)
      (Default|HideZoomOutPrompt _ui)
      (bind _output_get (Variables|Default|SetbExitThisCamera false))
      (Input|SetIgnoreMoveInput (Game|GetPlayerController (Game|GetPlayerState 0)) _output_get)
      (else
        (bind _asnwugame_mode (Utilities|Casting|CastToNWUGameMode (Game|GetGameMode)))
        (Variables|Default|SetPreviousCamera (Variables|/Game/Blueprints/NWUGameMode.NWUGameMode_C|GetCurrentCamera _asnwugame_mode))
        (CallFunction|SetThisCamera)
        (Default|HideZoominPrompt _ui_2)
        (Default|ShowZoomOutPrompt _ui_2)
        (bind _output_get_2 (Variables|Default|SetbExitThisCamera true))
        (Input|SetIgnoreMoveInput (Game|GetPlayerController (Game|GetPlayerState 0)) _output_get_2)))))

(fn ConstructionScript)