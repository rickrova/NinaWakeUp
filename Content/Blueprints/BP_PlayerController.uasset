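; Player controller that issues orders to the MayaNPCGuide dog companion (fetch, follow, retrieve, wait) and drives Nina's aimed throw.
; BeginPlay finds the dog and adds a spline, pooled spline meshes and a hit marker to the pawn.
; While aiming, the dog waits and Tick renders the predicted projectile path as scaled spline segments with a landing marker.
; Throwing launches through the character, sets the result as dog target and hides the preview.
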(event Custom|DrawPath
  (bind _returnvalue (Game|Player|GetPlayerPawn 0))
  (bind _splinemeshcomponents (Variables|Default|GetSplineMeshComponents))
  (bind _hitlocationmarker (Variables|Default|GetHitLocationMarker))
  (bind _pathsplinecomponent (Variables|Default|GetPathSplineComponent))
  (bind _returnvalue_2 (Utilities|Array|Length _splinemeshcomponents))
  (bind _returnvalue_3 (Math|Conversions|ToFloat(Integer) _returnvalue_2))
  (bind _asnina_character (Utilities|Casting|CastToNinaCharacter _returnvalue))
  (bind _output_get (Variables|Default|SetThrowVelocity (* (Math|Vector|Normalize (+ (* (Transformation|GetActorForwardVector _returnvalue) (- 1.0 (Variables|/Script/NinaProject.BaseCharacter|GetThrowForce _asnina_character))) (* (Variables|/Script/NinaProject.BaseCharacter|GetThrowForce _asnina_character) "0.000000,0.000000,1.000000"))) (* (Variables|/Script/NinaProject.BaseCharacter|GetThrowForce _asnina_character) 1.5e+03))))
  (bind (_outhit _outpathpositions) (Class|GameplayStatics|BlueprintPredictProjectilePathbyTraceChannel (+ (* (Transformation|GetActorForwardVector _returnvalue) 35.0) (Transformation|GetActorLocation _returnvalue)) _output_get true 0.0 "ECC_Visibility" false (Utilities|Array|MakeArray _returnvalue) "None"))
  (Transformation|SetWorldLocation _hitlocationmarker (.location _outhit) false false)
  (Rendering|SetVisibility _hitlocationmarker true false)
  (Spline|SetSplinePoints _pathsplinecomponent _outpathpositions "World" true)
  (for _index (range 0 (Variables|Default|GetThrowPathPiecesCount))
    (SplineMesh|SetStartandEnd (Utilities|Array|Get(acopy) _splinemeshcomponents _index) (.Location (Spline|GetLocationandTangentatSplinePoint _pathsplinecomponent _index "Local")) (.Tangent (Spline|GetLocationandTangentatSplinePoint _pathsplinecomponent _index "Local")) (.Location (Spline|GetLocationandTangentatSplinePoint _pathsplinecomponent (+ _index 1) "Local")) (.Tangent (Spline|GetLocationandTangentatSplinePoint _pathsplinecomponent (+ _index 1) "Local")) true :!class /Script/Engine.SplineMeshComponent)
    (SplineMesh|SetStartScale (Utilities|Array|Get(acopy) _splinemeshcomponents _index) (Math|Vector2D|MakeVector2D (Math|Float|Clamp(Float) (* (/ (Math|Conversions|ToFloat(Integer) _index) _returnvalue_3) 1e+01) 0.1 1.5) (Math|Float|Clamp(Float) (* (/ (Math|Conversions|ToFloat(Integer) _index) _returnvalue_3) 1e+01) 0.1 1.5)) true :!class /Script/Engine.SplineMeshComponent)
    (SplineMesh|SetEndScale (Utilities|Array|Get(acopy) _splinemeshcomponents _index) (Math|Vector2D|MakeVector2D (Math|Float|Clamp(Float) (* (/ (+ (Math|Conversions|ToFloat(Integer) _index) 1.0) _returnvalue_3) 1e+01) 0.1 1.5) (Math|Float|Clamp(Float) (* (/ (+ (Math|Conversions|ToFloat(Integer) _index) 1.0) _returnvalue_3) 1e+01) 0.1 1.5)) true :!class /Script/Engine.SplineMeshComponent)
    (if (> _index (Math|Integer|Min(Integer) (- (Spline|GetNumberOfSplinePoints (Variables|Default|GetPathSplineComponent)) 2) (Utilities|Array|Length (Variables|Default|GetSplineMeshComponents))))
      (Rendering|SetVisibility (Utilities|Array|Get(acopy) _splinemeshcomponents _index) false false)
      (else
        (Rendering|SetVisibility (Utilities|Array|Get(acopy) _splinemeshcomponents _index) true false)))))

(event EventBeginPlay
  (bind _returnvalue (Game|Player|GetPlayerPawn 0))
  (bind _outactors (Actor|GetAllActorsOfClass "/Game/Blueprints/NavigationSystem/MayaNPCGuide.MayaNPCGuide_C"))
  (Variables|Default|SetDog (Utilities|Array|Get(acopy) _outactors))
  (bind _returnvalue_2 (AddComponent|AddSplineComponent _returnvalue false))
  (bind _output_get (Variables|Default|SetPathSplineComponent _returnvalue_2))
  (for _index (range 0 (Variables|Default|GetThrowPathPiecesCount))
    (Class|SplineComponent|AddPoint _output_get (Utilities|Struct|MakeSplinePoint 0.0 "0.000000,0.000000,0.000000" "0.000000,0.000000,0.000000" "0.000000,0.000000,0.000000" "0.000000,0.000000,0.000000" "1.000000,1.000000,1.000000" "Curve") false)
    (bind _returnvalue_3 (AddComponent|AddSplineMeshComponent _returnvalue false))
    (Rendering|SetVisibility _returnvalue_3 false false)
    (Rendering|SetCastShadow _returnvalue_3 false)
    (Utilities|Array|Add (Variables|Default|GetSplineMeshComponents) _returnvalue_3))
  (bind _returnvalue_4 (AddComponent|AddStaticMeshComponent _returnvalue false))
  (bind _output_get_2 (Variables|Default|SetHitLocationMarker _returnvalue_4))
  (Rendering|SetVisibility _output_get_2 false false)
  (Rendering|SetCastShadow _output_get_2 false)
  (Rendering|SetRenderCustomDepth _returnvalue_4 true))

(event EventTick
  (params (DeltaSeconds :type Float%20%28single-precision%29))
  (if (Variables|Default|GetbDrawingPath)
    (CallFunction|DrawPath)))

(event EventAim
  (Default|Wait (Variables|Default|GetDog))
  (for _array_element (Variables|Default|GetSplineMeshComponents)
    (Rendering|SetVisibility _array_element true false))
  (Variables|Default|SetbDrawingPath true))

(event EventUpOrder
  (Default|Fetch (Variables|Default|GetDog)))

(event EventRightOrder
  (Default|Retrieve (Variables|Default|GetDog))
  (Development|PrintString "trying to retrieve"))

(event EventLeftOrder
  (Default|Follow (Variables|Default|GetDog))
  (Development|PrintString "trying to follow"))

(event EventDownOrder
  (Default|Wait (Variables|Default|GetDog)))

(event EventThrow
  (bind _asnina_character_bp (Utilities|Casting|CastToNinaCharacter_BP (Game|GetPlayerCharacter 0)))
  (bind _thrownitem (Default|Throw _asnina_character_bp (Variables|Default|GetThrowVelocity)))
  (Variables|/Game/Blueprints/NavigationSystem/MayaNPCGuide.MayaNPCGuide_C|SetTarget (Variables|Default|GetDog) _thrownitem)
  (Rendering|SetVisibility (Variables|Default|GetHitLocationMarker) false false)
  (for _array_element (Variables|Default|GetSplineMeshComponents)
    (Rendering|SetVisibility _array_element false false))
  (Variables|Default|SetbDrawingPath false))

(fn ConstructionScript)