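; ItemReceiver_BP is an interactable that waits for a specific inventory item from the player.
; Overlapping its collision component switches HUD prompts and registers or clears it as NinaCharacter_BP's Interactable.
; Interact compares the equipped or passed item's name to its required item.
; A match notifies ActionReceiver (the GameMode for Dream responses) and unlocks a HUD drawing; a mismatch calls SwitchMenu on the player controller.
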(event OnComponentEndOverlap(CollisionComponent)
  (params (OverlappedComponent :type Primitive%20Component%20Object%20Reference) (OtherActor :type Actor%20Object%20Reference) (OtherComp :type Primitive%20Component%20Object%20Reference) (OtherBodyIndex :type Integer))
  (bind _returnvalue (Game|GetPlayerCharacter 0))
  (if (== OtherActor _returnvalue)
    (Class|InteractionInterfaceBP|SwitchPromptRequest(Message) (HUD|GetHUD (Game|GetPlayerController 0)) "NewEnumerator5" "NewEnumerator4" false)
    (bind _asnina_character_bp (Utilities|Casting|CastToNinaCharacter_BP _returnvalue))
    (Variables|/Game/Characters/Nina/NinaCharacter_BP.NinaCharacter_BP_C|SetInteractable _asnina_character_bp 0)))

(event OnComponentBeginOverlap(CollisionComponent)
  (params (OverlappedComponent :type Primitive%20Component%20Object%20Reference) (OtherActor :type Actor%20Object%20Reference) (OtherComp :type Primitive%20Component%20Object%20Reference) (OtherBodyIndex :type Integer) (bFromSweep :type Boolean) (SweepResult :type Hit%20Result%20Structure%20%28by%20ref%29))
  (bind _returnvalue (Game|GetPlayerCharacter 0))
  (if (Variables|Default|GetCanInteract)
    (if (== OtherActor _returnvalue)
      (Class|InteractionInterfaceBP|SwitchPromptRequest(Message) (HUD|GetHUD (Game|GetPlayerController 0)) "NewEnumerator4" "NewEnumerator5" false)
      (bind _asnina_character_bp (Utilities|Casting|CastToNinaCharacter_BP _returnvalue))
      (Variables|/Game/Characters/Nina/NinaCharacter_BP.NinaCharacter_BP_C|SetInteractable _asnina_character_bp self))))

(event EventBeginPlay
  (Variables|Default|SetItemMeta (Variables|/Script/NinaProject.Item|GetMetaData (Variables|Default|GetItem)))
  (switch Utilities|FlowControl|Switch|SwitchonInteractionResponseType (Variables|Default|GetInteractionResponseType)
    (:NewEnumerator1
      (Variables|Default|SetActionReceiver (Game|GetGameMode)))))

(event EventInteract
  (params (Param :type Object%20Object%20Reference))
  (bind _returnvalue (Game|GetPlayerController 0))
  (bind _itemmeta (Variables|Default|GetItemMeta))
  (if (Variables|Default|GetCanInteract)
    (bind _asbase_player_controller (Utilities|Casting|CastToBasePlayerController _returnvalue))
    (if (== Param 0)
      (bind _asnwugame_mode (Utilities|Casting|CastToNWUGameMode (Game|GetGameMode)))
      (if (Utilities|Enum|Equal(Enum) (.name (Variables|/Script/NinaProject.Inventory|GetEquippedItem (Variables|/Script/NinaProject.NinaProjectGameModeBase|GetInventory _asnwugame_mode))) (.name _itemmeta))
        (Development|PrintString (Utilities|String|Append "nombres: " (Utilities|String|ToString(Text) (.name (Variables|/Script/NinaProject.Inventory|GetEquippedItem (Variables|/Script/NinaProject.NinaProjectGameModeBase|GetInventory _asnwugame_mode)))) " y " (Utilities|String|ToString(Text) (.name _itemmeta))))
        (Class|InteractionInterfaceBP|SwitchPromptRequest(Message) (HUD|GetHUD _returnvalue) "NewEnumerator9" "NewEnumerator5" true :!label _label)
        (Class|InteractableVolumeInterface|InteractionResponse(Message) (Variables|Default|GetActionReceiver) (Variables|Default|GetItemMeta))
        (bind _asnwuhud_bp (Utilities|Casting|CastToNWUHUD_BP (HUD|GetHUD (Game|GetPlayerController 0))))
        (Default|UnlockDraw _asnwuhud_bp (Variables|Default|GetUlockableDrawIndex))
        (else
          (Class|BasePlayerController|SwitchMenu _asbase_player_controller :!label _label_2)))
      (else
        (bind _asuitem_data (Utilities|Casting|CastToUItemData Param))
        (if (Utilities|Enum|Equal(Enum) (.name (Variables|/Game/HUD/UItemData.UItemData_C|GetItemData _asuitem_data)) (.name (Variables|Default|GetItemMeta)))
          (Development|PrintString "sended")
          (goto _label)
          (else
            (goto _label_2)))))))

(fn ConstructionScript)