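; InfoActor is an actor that trails the player character's InfoSlot component, facing relative to the player's camera.
; On BeginPlay it casts player character 0 to NinaCharacter_BP and caches its InfoSlot.
; Each Tick it eases its location toward the slot and its yaw toward the camera yaw plus a 90-degree offset, keeping roll and pitch, using delta-scaled lerps and teleporting moves.
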(event EventBeginPlay
  (bind _asnina_character_bp (Utilities|Casting|CastToNinaCharacter_BP (Game|GetPlayerCharacter 0)))
  (Variables|Default|SetInfoSlot (Variables|/Game/Characters/Nina/NinaCharacter_BP.NinaCharacter_BP_C|GetInfoSlot _asnina_character_bp)))

(event Collision|EventActorBeginOverlap
  (params (OtherActor :type Actor%20Object%20Reference)))

(event EventTick
  (params (DeltaSeconds :type Float%20%28single-precision%29))
  (bind _returnvalue (Transformation|GetActorRotation))
  (bind _returnvalue_2 (* DeltaSeconds 5.0))
  (Transformation|SetActorLocationAndRotation (Math|Vector|Lerp(Vector) (Transformation|GetActorLocation) (Transformation|GetWorldLocation (Variables|Default|GetInfoSlot)) _returnvalue_2) (Math|Rotator|Lerp(Rotator) (Math|Rotator|MakeRotator (.roll _returnvalue) (.pitch _returnvalue) (.yaw _returnvalue)) (Math|Rotator|MakeRotator (.roll _returnvalue) (.pitch _returnvalue) (+ (.yaw (Transformation|GetWorldRotation (Variables|/Script/NinaProject.BaseCharacter|GetCamera (stale EventBeginPlay _asnina_character_bp)))) 9e+01)) _returnvalue_2 true) false true))

(fn ConstructionScript)