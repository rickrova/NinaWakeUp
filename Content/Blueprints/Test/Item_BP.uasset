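; Item_BP is a pickup actor that the player collects into the inventory through interaction.
; When the player character overlaps its Collision, it switches the HUD prompt and registers itself as NinaCharacter_BP's Interactable.
; End overlap reverses the prompt switch but leaves that Interactable reference set.
; Interact adds the item's MetaData to the NWUGameMode Inventory, then destroys the actor.
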(event OnComponentBeginOverlap(Collision)
  (params (OverlappedComponent :type Primitive%20Component%20Object%20Reference) (OtherActor :type Actor%20Object%20Reference) (OtherComp :type Primitive%20Component%20Object%20Reference) (OtherBodyIndex :type Integer) (bFromSweep :type Boolean) (SweepResult :type Hit%20Result%20Structure%20%28by%20ref%29))
  (bind _returnvalue (Game|GetPlayerCharacter 0))
  (if (== OtherActor _returnvalue)
    (Class|InteractionInterfaceBP|SwitchPromptRequest(Message) (HUD|GetHUD (Game|GetPlayerController 0)) "NewEnumerator0" "NewEnumerator5" false)
    (bind _asnina_character_bp (Utilities|Casting|CastToNinaCharacter_BP _returnvalue))
    (Variables|/Game/Characters/Nina/NinaCharacter_BP.NinaCharacter_BP_C|SetInteractable _asnina_character_bp self)))

(event OnComponentEndOverlap(Collision)
  (params (OverlappedComponent :type Primitive%20Component%20Object%20Reference) (OtherActor :type Actor%20Object%20Reference) (OtherComp :type Primitive%20Component%20Object%20Reference) (OtherBodyIndex :type Integer))
  (if (== OtherActor (Game|GetPlayerCharacter 0))
    (Class|InteractionInterfaceBP|SwitchPromptRequest(Message) (HUD|GetHUD (Game|GetPlayerController 0)) "NewEnumerator5" "NewEnumerator0" false)))

(event EventInteract
  (params (Param :type Object%20Object%20Reference))
  (bind _asnwugame_mode (Utilities|Casting|CastToNWUGameMode (Game|GetGameMode)))
  (Class|Inventory|AddtoInventory (Variables|/Script/NinaProject.NinaProjectGameModeBase|GetInventory _asnwugame_mode) (Variables|Default|GetMetaData))
  (Actor|DestroyActor))

(fn ConstructionScript)