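; Notebook item that displays drawings as flippable two-page spreads, using drawing indices read from the HUD at BeginPlay.
; Four dynamic page materials hold the current and next spread, with a fallback texture when the fourth drawing is invalid.
; PadRight and PadLeft update the page index and textures, then play the page-turn animation forward or in reverse.
; A short delay lock prevents overlapping turns.
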(event EventBeginPlay
  (bind _returnvalue (Rendering|Material|CreateDynamicMaterialInstance 1 "/Game/Materials/Items/Page_MI.Page_MI" "Page1" :!class /Script/Engine.PrimitiveComponent))
  (Rendering|Material|SetMaterial 1 _returnvalue)
  (Variables|Default|SetPage1 _returnvalue)
  (bind _returnvalue_2 (Rendering|Material|CreateDynamicMaterialInstance 4 "/Game/Materials/Items/Page_MI.Page_MI" "Page2" :!class /Script/Engine.PrimitiveComponent))
  (Rendering|Material|SetMaterial 4 _returnvalue_2)
  (Variables|Default|SetPage2 _returnvalue_2)
  (bind _returnvalue_3 (Rendering|Material|CreateDynamicMaterialInstance 3 "/Game/Materials/Items/Page_MI.Page_MI" "Page3" :!class /Script/Engine.PrimitiveComponent))
  (Rendering|Material|SetMaterial 3 _returnvalue_3)
  (Variables|Default|SetPage3 _returnvalue_3)
  (bind _returnvalue_4 (Rendering|Material|CreateDynamicMaterialInstance 2 "/Game/Materials/Items/Page_MI.Page_MI" "Page4" :!class /Script/Engine.PrimitiveComponent))
  (Rendering|Material|SetMaterial 2 _returnvalue_4)
  (Variables|Default|SetPage4 _returnvalue_4)
  (bind _asnwuhud_bp (Utilities|Casting|CastToNWUHUD_BP (HUD|GetHUD (Game|GetPlayerController 0))))
  (Variables|Default|SetIndexes (Variables|/Game/HUD/NWUHUD_BP.NWUHUD_BP_C|GetDrawsIndices _asnwuhud_bp))
  (CallFunction|SetImages))

(event EventPadRight
  (if (and (< (Variables|Default|GetCurrentPage) (/ (- (Utilities|Array|Length (Variables|Default|GetIndexes)) 1) 2)) (Variables|Default|GetCanTurnPage))
    (CallFunction|SetImages)
    (Variables|Default|SetCurrentPage (+ (Variables|Default|GetCurrentPage) 1))
    (Components|Timeline|SetPlayRate 5.0)
    (Components|Animation|SetPosition 0.0 false)
    (Audio|Components|Audio|Play false)
    (Variables|Default|SetCanTurnPage false)
    (Utilities|FlowControl|Delay 0.4)
    (Variables|Default|SetCanTurnPage true)))

(event EventPadLeft
  (if (and (> (Variables|Default|GetCurrentPage) 0) (Variables|Default|GetCanTurnPage))
    (Variables|Default|SetCurrentPage (+ (Variables|Default|GetCurrentPage) -1))
    (CallFunction|SetImages)
    (Components|Timeline|SetPlayRate -5.0)
    (Components|Animation|SetPosition 2.46 false)
    (Audio|Components|Audio|Play false)
    (Variables|Default|SetCanTurnPage false)
    (Utilities|FlowControl|Delay 0.4)
    (Variables|Default|SetCanTurnPage true)))

(fn SetImages
  (bind _currentpage (Variables|Default|GetCurrentPage))
  (bind _indexes (Variables|Default|GetIndexes))
  (bind _page4 (Variables|Default|GetPage4))
  (bind _indexes_2 (Variables|Default|GetIndexes))
  (bind _draws (Variables|Default|GetDraws))
  (bind _returnvalue (* _currentpage 2))
  (bind _output (Utilities|Array|Get(acopy) _indexes_2 _returnvalue))
  (bind _returnvalue_2 (+ _returnvalue 3))
  (bind _output_2 (Utilities|Array|Get(acopy) _indexes _returnvalue_2))
  (bind _output_3 (Utilities|Array|Get(acopy) _draws _output_2))
  (Rendering|Material|SetTextureParameterValue (Variables|Default|GetPage1) "Draw" (Utilities|Array|Get(acopy) (Variables|Default|GetDraws) _output))
  (Rendering|Material|SetTextureParameterValue (Variables|Default|GetPage2) "Draw" (Utilities|Array|Get(acopy) (Variables|Default|GetDraws) (Utilities|Array|Get(acopy) (Variables|Default|GetIndexes) (+ _returnvalue 1))))
  (Rendering|Material|SetTextureParameterValue (Variables|Default|GetPage3) "Draw" (Utilities|Array|Get(acopy) (Variables|Default|GetDraws) (Utilities|Array|Get(acopy) (Variables|Default|GetIndexes) (+ _returnvalue 2))))
  (Utilities|IsValid _output_3
    (:Is%20Valid
      (Rendering|Material|SetTextureParameterValue _page4 "Draw" _output_3))
    (:Is%20Not%20Valid
      (Rendering|Material|SetTextureParameterValue _page4 "Draw" "/Game/Textures/Whiter.Whiter")))
  (Development|PrintString (Utilities|String|ToString(Integer) _output)))