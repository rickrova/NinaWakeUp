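; Hazard actor that deals one point of damage to the Nina character on overlap, unless she is invincible.
; Begin overlap stores the character reference, sets an InsideDamage flag and runs the damage check, while end overlap clears the flag.
; The CheckDamage event exposes the same check, so damage can be re-applied while she remains inside; nothing in this Blueprint calls that event.
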(event Custom|CheckDamage
  (if (and (not (Variables|/Script/NinaProject.BaseCharacter|GetbInvincible (stale Collision|EventActorBeginOverlap _asnina_character_bp))) (Variables|Default|GetInsideDamage))
    (Default|OnDamage (stale Collision|EventActorBeginOverlap _asnina_character_bp) self 1)))

(event EventBeginPlay)

(event Collision|EventActorBeginOverlap
  (params (OtherActor :type Actor%20Object%20Reference))
  (bind _asnina_character_bp (Utilities|Casting|CastToNinaCharacter_BP OtherActor))
  (Variables|Default|SetInsideDamage true)
  (if (and (not (Variables|/Script/NinaProject.BaseCharacter|GetbInvincible _asnina_character_bp)) (Variables|Default|GetInsideDamage))
    (Default|OnDamage _asnina_character_bp self 1)))

(event EventTick
  (params (DeltaSeconds :type Float%20%28single-precision%29)))

(event Collision|EventActorEndOverlap
  (params (OtherActor :type Actor%20Object%20Reference))
  (Utilities|Casting|CastToNinaCharacter_BP OtherActor)
  (Variables|Default|SetInsideDamage false))

(fn ConstructionScript)