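; Forest turret that scans by rotating its cannon and fires pooled projectiles at the player character.
; Inside the sight sphere, a view-angle or proximity check plus a line trace starts tracking with clamped pitch.
; An aligned cannon enters a faster-turning, timed danger state and fires round-robin from projectiles spawned at BeginPlay, pausing between shots.
; StopFire blocks firing and reinitializes all projectiles except the instigator until ResumeFire re-enables it.
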(event Custom|Fire
  (if (Variables|Default|GetbCanFire)
    (Variables|Default|SetbBusy true)
    (Default|Fire (Utilities|Array|Get(acopy) (Variables|Default|GetProjectiles) (Variables|Default|GetCurrentProjectile)) (Math|Vector|Normalize (- (Variables|Default|GetNinaLocation) (Transformation|GetWorldLocation (Variables|Default|GetNozzle)))) (Variables|Default|GetProjectileVelocity) (Transformation|GetWorldLocation (Variables|Default|GetNozzle)))
    (if (<= (+ (Variables|Default|GetCurrentProjectile) 1) (Variables|Default|GetProjectilesPoll))
      (Variables|Default|SetCurrentProjectile (+ (Variables|Default|GetCurrentProjectile) 1))
      (else
        (Variables|Default|SetCurrentProjectile 0)))
    (Utilities|Time|SetTimerbyEvent (delegate Custom|ResetBusy) (Variables|Default|GetRestoreTime))))

(event Custom|ResumeFire
  (Variables|Default|SetbCanFire true))

(event Custom|ResetBusy
  (Variables|Default|SetbBusy false))

(event Custom|ResetDanger
  (Variables|Default|SetbDanger false))

(event Custom|StopFire
  (params (Instigator :type Projectile%20Object%20Reference))
  (Variables|Default|SetbCanFire false)
  (for _array_element (Variables|Default|GetProjectiles)
    (if (not (== _array_element Instigator))
      (Default|Init _array_element (Transformation|GetWorldLocation (Variables|Default|GetBase))))))

(event EventBeginPlay
  (bind _base (Variables|Default|GetBase))
  (bind _returnvalue (Transformation|GetWorldLocation _base))
  (for _index (range 0 (Variables|Default|GetProjectilesPoll))
    (bind _returnvalue_2 (Game|SpawnActorfromClass "/Game/Blueprints/ForestBlueprints/Projectile.Projectile_C" (Math|Transform|MakeTransform _returnvalue "0, 0, 0" "0.100000,0.100000,0.100000") "AlwaysSpawn" self 0))
    (Default|Init _returnvalue_2 _returnvalue)
    (Utilities|Array|Add (Variables|Default|GetProjectiles) _returnvalue_2))
  (Components|Sphere|SetSphereRadius (Variables|Default|GetSightArea) (Variables|Default|GetSightLength) true))

(event Collision|EventActorBeginOverlap
  (params (OtherActor :type Actor%20Object%20Reference))
  (if (== OtherActor (Game|GetPlayerCharacter 0))
    (Variables|Default|SetbInSight true)
    (Variables|Default|SetCurrentRotationSpeed (Variables|Default|GetInitialRotationSpeed))
    (Variables|Default|SetbDanger false)
    (Utilities|Time|ClearandInvalidateTimerbyHandle (stale EventTick _returnvalue_3))))

(event EventTick
  (params (DeltaSeconds :type Float%20%28single-precision%29))
  (bind _cannon (Variables|Default|GetCannon))
  (bind _cannon_2 (Variables|Default|GetCannon))
  (bind _cannon_3 (Variables|Default|GetCannon))
  (bind _returnvalue (Transformation|GetWorldRotation _cannon_2))
  (bind _returnvalue_2 (Transformation|GetWorldLocation _cannon))
  (if (not (Variables|Default|GetbBusy))
    (if (Variables|Default|GetbInSight)
      (bind _output_get (Variables|Default|SetNinaLocation (Transformation|GetActorLocation (Game|GetPlayerCharacter 0))))
      (bind _output_get_2 (Variables|Default|SetVectorToNina (- _output_get (Transformation|GetWorldLocation (Variables|Default|GetCannon)))))
      (Variables|Default|SetAngleTo%20Nina (Class|KismetMathLibrary|DegAcos (Math|Vector|DotProduct (Math|Vector|Normalize _output_get_2) (Math|Vector|GetForwardVector (Variables|Default|GetCannon)))))
      (if (Variables|Default|GetbDanger)
        (bind _outhit (Collision|LineTraceByChannel _returnvalue_2 (+ _returnvalue_2 (* (Math|Vector|Normalize (Variables|Default|GetVectorToNina)) (Variables|Default|GetSightLength))) "TraceTypeQuery1" false 0 "ForOneFrame" true "(R=1.000000,G=0.766184,B=0.000000,A=1.000000)" "(R=0.000000,G=1.000000,B=0.000000,A=1.000000)" 0.1 :!label _label))
        (if (== (.hitactor _outhit) (Game|GetPlayerCharacter 0))
          (Transformation|SetWorldRotation _cannon_3 (Math|Rotator|MakeRotator (.roll (Math|Rotator|Lerp(Rotator) (Transformation|GetWorldRotation _cannon_3) (Math|Rotator|MakeRotfromX (Math|Vector|Normalize (Variables|Default|GetVectorToNina))) (* DeltaSeconds (Variables|Default|GetCurrentRotationSpeed)) true)) (Math|Float|Clamp(Float) (.pitch (Math|Rotator|Lerp(Rotator) (Transformation|GetWorldRotation _cannon_3) (Math|Rotator|MakeRotfromX (Math|Vector|Normalize (Variables|Default|GetVectorToNina))) (* DeltaSeconds (Variables|Default|GetCurrentRotationSpeed)) true)) -3e+01 3e+01) (.yaw (Math|Rotator|Lerp(Rotator) (Transformation|GetWorldRotation _cannon_3) (Math|Rotator|MakeRotfromX (Math|Vector|Normalize (Variables|Default|GetVectorToNina))) (* DeltaSeconds (Variables|Default|GetCurrentRotationSpeed)) true))) false true)
          (if (< (Variables|Default|GetAngleTo%20Nina) (Variables|Default|GetFireAngleThereshold))
            (Variables|Default|SetbDanger true)
            (Variables|Default|SetCurrentRotationSpeed (Variables|Default|GetDangerRotationSpeed))
            (CallFunction|Fire)
            (goto _label_3 Reset))
          (else
            (if (Variables|Default|GetbDanger) :!label _label_2
              (Utilities|FlowControl|DoOnce false :!label _label_3
                (:Completed
                  (bind _returnvalue_3 (Utilities|Time|SetTimerbyEvent (delegate Custom|ResetDanger) (Variables|Default|GetDangerTime)))))
              (else
                (Transformation|AddRelativeRotation _cannon_2 "0,1.000000, 0" false false :!label _label_4)
                (Transformation|SetWorldRotation _cannon_2 (Math|Rotator|MakeRotator (.roll _returnvalue) (Math|Float|Lerp (.pitch _returnvalue) 0.0 (* (Utilities|Time|GetWorldDeltaSeconds) 5.0)) (.yaw _returnvalue)) false false)
                (Variables|Default|SetbDanger false)
                (Variables|Default|SetCurrentRotationSpeed (Variables|Default|GetInitialRotationSpeed))))))
        (elif (or (< (Variables|Default|GetAngleTo%20Nina) (Variables|Default|GetSightAngle)) (< (Math|Vector|VectorLength (Variables|Default|GetVectorToNina)) (Variables|Default|GetDangerDistance)))
          (goto _label)
          (else
            (goto _label_4))))
      (else
        (goto _label_2)))))

(event Collision|EventActorEndOverlap
  (params (OtherActor :type Actor%20Object%20Reference))
  (if (== OtherActor (Game|GetPlayerCharacter 0))
    (Variables|Default|SetbInSight false)))

(fn ConstructionScript)