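; Pooled turret projectile that Fire launches from a given location and Init parks, inactive and collisionless, at a storage location for reuse.
; Tick moves it by swept steps along its direction until it hits something, then it bounces off under physics and returns to storage a second later.
; Hitting NinaCharacter_BP also calls StopFire on the owning Turret and, unless already hit, triggers her hit animation, ignores move input and knocks her back.
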(event OnComponentHit(Sphere)
  (params (HitComponent :type Primitive%20Component%20Object%20Reference) (OtherActor :type Actor%20Object%20Reference) (OtherComp :type Primitive%20Component%20Object%20Reference) (NormalImpulse :type Vector :default "0, 0, 0") (Hit :type Hit%20Result%20Structure%20%28by%20ref%29))
  (bind _sphere (Variables|Default|GetSphere))
  (bind _asnina_character_bp (Utilities|Casting|CastToNinaCharacter_BP OtherActor)
    (:then
      (bind _asturret (Utilities|Casting|CastToTurret (Components|GetOwner)))
      (Default|StopFire _asturret self)
      (bind _asnina_animation_bp (Default|GetAnimationBlueprint _asnina_character_bp))
      (if (Variables|/Game/Characters/Nina/Animations/Nina_Animation_BP.Nina_Animation_BP_C|GetbHit _asnina_animation_bp)
        _
        (else
          (Default|OnHit _asnina_animation_bp self)
          (Input|SetIgnoreMoveInput (Pawn|GetController _asnina_character_bp) true)
          (Transformation|SetActorRotation _asnina_character_bp (Math|Rotator|MakeRotator (.roll (Transformation|GetActorRotation _asnina_character_bp)) (.pitch (Transformation|GetActorRotation _asnina_character_bp)) (.yaw (Math|Rotator|MakeRotfromX (.impactnormal Hit)))) true)
          (Physics|AddImpulse (Variables|/Script/Engine.Character|GetCharacterMovement _asnina_character_bp) (* (Math|Vector|Normalize (+ (* (.impactnormal Hit) -1.0) "0, 0,0.100000")) 5e+02) true))))
    (:CastFailed
      _))
  (Transformation|SetWorldLocation (Variables|Default|GetSphere) (+ (.location Hit) (* (.impactnormal Hit) 2e+01)) false true)
  (Physics|SetSimulatePhysics _sphere true)
  (Physics|SetPhysicsLinearVelocity _sphere (* (+ (.impactnormal Hit) "0, 0,2.000000") 1e+02) false "None")
  (Actor|Tick|SetActorTickEnabled false)
  (bind _returnvalue (Utilities|Time|SetTimerbyEvent (delegate Custom|InitBridge) 1.0)))

(event Custom|Fire
  (params (Direction :type Vector) (Velocity :type Float%20%28single-precision%29) (InitialFireLocation :type Vector))
  (bind _sphere (Variables|Default|GetSphere))
  (if (Variables|Default|GetbActive)
    (CallFunction|Init (Variables|Default|GetStoreLocation))
    (Utilities|Time|ClearandInvalidateTimerbyHandle (stale OnComponentHit(Sphere) _returnvalue)))
  (Transformation|SetActorLocation InitialFireLocation false true)
  (Variables|Default|SetDirection Direction)
  (Variables|Default|SetVelocity Velocity)
  (bind _output_get (Variables|Default|SetbActive true))
  (Actor|Tick|SetActorTickEnabled _output_get)
  (Collision|SetCollisionEnabled _sphere "QueryAndPhysics")
  (Collision|SetCollisionResponsetoAllChannels _sphere "ECR_Block"))

(event Custom|Init
  (params (StoreLocation :type Vector))
  (bind _sphere (Variables|Default|GetSphere))
  (bind _output_get (Variables|Default|SetStoreLocation StoreLocation))
  (Transformation|SetActorLocation _output_get false false)
  (bind _output_get_2 (Variables|Default|SetbActive false))
  (Actor|Tick|SetActorTickEnabled _output_get_2)
  (Physics|SetSimulatePhysics _sphere false)
  (Collision|SetCollisionEnabled (Variables|Default|GetSphere) "NoCollision")
  (Collision|SetCollisionResponsetoAllChannels _sphere "ECR_Ignore")
  (Utilities|Time|ClearandInvalidateTimerbyHandle (stale OnComponentHit(Sphere) _returnvalue)))

(event Custom|InitBridge
  (if (Variables|Default|GetbActive)
    (CallFunction|Init (Variables|Default|GetStoreLocation))))

(event EventBeginPlay)

(event Collision|EventActorBeginOverlap
  (params (OtherActor :type Actor%20Object%20Reference)))

(event EventTick
  (params (DeltaSeconds :type Float%20%28single-precision%29))
  (Transformation|SetActorLocation (+ (* (Variables|Default|GetDirection) (* DeltaSeconds (Variables|Default|GetVelocity))) (Transformation|GetActorLocation)) true false))

(fn ConstructionScript)