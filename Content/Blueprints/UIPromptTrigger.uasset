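; UI prompt trigger actor that switches panels on the game's Widgo UI when something overlaps its Collision component.
; On BeginPlay it binds to the NWUGameMode's OnCreateUI event and caches the Widgo reference once that fires.
; Any begin overlap calls SwitchPanels with the same enum entry as in and out panel.
; End overlap and Interact handling are empty stubs, and the nodes setting CanInteract are disconnected.
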(event OnComponentBeginOverlap(Collision)
  (params (OverlappedComponent :type Primitive%20Component%20Object%20Reference) (OtherActor :type Actor%20Object%20Reference) (OtherComp :type Primitive%20Component%20Object%20Reference) (OtherBodyIndex :type Integer) (bFromSweep :type Boolean) (SweepResult :type Hit%20Result%20Structure%20%28by%20ref%29))
  (Default|SwitchPanels (Variables|Default|GetWidgo) "NewEnumerator5" "NewEnumerator5"))

(event OnComponentEndOverlap(Collision)
  (params (OverlappedComponent :type Primitive%20Component%20Object%20Reference) (OtherActor :type Actor%20Object%20Reference) (OtherComp :type Primitive%20Component%20Object%20Reference) (OtherBodyIndex :type Integer)))

(event Custom|OnCreateUIHandrer
  (Variables|Default|SetWidgo (Variables|/Game/Blueprints/NWUGameMode.NWUGameMode_C|GetWidgo (stale EventBeginPlay _asnwugame_mode)))
  (Development|PrintString "referenced "))

(event EventBeginPlay
  (bind _asnwugame_mode (Utilities|Casting|CastToNWUGameMode (Game|GetGameMode)))
  (EventDispatchers|BindEventtoOnCreateUI _asnwugame_mode (delegate Custom|OnCreateUIHandrer)))

(event Collision|EventActorBeginOverlap
  (params (OtherActor :type Actor%20Object%20Reference)))

(event EventTick
  (params (DeltaSeconds :type Float%20%28single-precision%29)))

(event EventInteract
  (params (Param :type Object%20Object%20Reference)))

(event Input|ActionEvents|InputActionInteract
  (params (Key :type Key%20Structure :default "None"))
  (:Pressed
    (if (Variables|Default|GetbCanInteract)
      _)))

(fn ConstructionScript)